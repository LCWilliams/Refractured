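; Static laser emitter that fires a coloured, bouncing beam from its arrow through a laser component and particle effect.
; A looping timeline replaces Tick, re-firing at a rate set by PerformanceDelay.
; When NeedsPower is set, it fires only while all referenced receivers are active, otherwise hiding the beam.
; A RaycastHitCheckM macro, not called in the event graph, toggles hit laser switches and passes them the beam colour.
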(event EventBeginPlay
  (bind _bp_cb_laser_component_01 (Variables|Default|GetBP_CB_Laser_Component_01))
  (bind _ps_lw_laserbeam_00 (Variables|Default|GetPS_LW_LaserBeam_00))
  ;[1 1 1] Initialise Components
  (Utilities|FlowControl|Sequence
    (:then_0
      (Components|Activation|SetActive _ps_lw_laserbeam_00 false false)
      (Default|TraceSetup _bp_cb_laser_component_01 (Variables|Default|GetArrow)))
    (:then_1
      ;[1 1 1] Event Tick Replacer
      (Components|Timeline|SetPlayRate (Variables|Default|GetLooping) (Variables|Default|GetPerformanceDelay))
      (Timeline|Looping PlayFromStart
        (:NewTrack_1
          ;[1 1 1] Raycast
          (if (Variables|Activation|GetNeedsPower)
            (bind _recievers (CallFunction|ReciverChecker))
            (if _recievers
              (Default|FireLaser _bp_cb_laser_component_01 (Variables|Default|GetArrow) (Variables|Laser|GetLaserColour) (Variables|Default|GetPS_LW_LaserBeam_00) (Variables|Default|GetMaxBounce) :!label _label)
              (else
                (Components|Activation|SetActive _ps_lw_laserbeam_00 false false)))
            (else
              (goto _label))))))))

(fn ConstructionScript)

(fn ReciverChecker
  (bind _receiverref (Variables|Activation|GetReceiverRef))
  (Variables|Default|SetActivated 0)
  (for _array_element _receiverref
    (if (Variables|/Game/Blueprints/Parents/BP_CB_ParentDontUse_00.BP_CB_ParentDontUse_00_C|GetisActive _array_element)
      (bind _result (Math|Integer|IncrementInt (Variables|Default|GetActivated))
        (:%20%20
          (Variables|Default|SetActivated _result)))
      (else
        (Variables|Default|SetActivated 0))))
  (return (>= (Variables|Default|GetActivated) (Utilities|Array|Length _receiverref))))