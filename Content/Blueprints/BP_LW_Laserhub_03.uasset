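; Laser hub actor that fires a coloured particle beam from its arrow while its activatable component is switched on.
; Each tick a visibility trace sets the beam endpoint and passes the colour to the raycast component of "LaserActivatable" hits.
; "Reflective" hits spawn one mirrored trace that can also activate targets but does not extend the beam.
; Switching off disables the emitters and sends NotActive to the last direct hit if anything was activated.
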(event EventTick
  (params (DeltaSeconds :type Float%20%28single-precision%29))
  (bind _ps_lw_laserbeam_00 (Variables|Default|GetPS_LW_LaserBeam_00))
  (bind _arrow (Variables|Default|GetArrow))
  (bind _returnvalue (Transformation|GetWorldLocation _arrow))
  (bind _returnvalue_2 (Transformation|GetWorldRotation _arrow))
  (bind _returnvalue_3 (Math|Vector|GetForwardVector _returnvalue_2))
  (bind _returnvalue_4 (* _returnvalue_3 1e+04))
  (bind _returnvalue_5 (+ _returnvalue _returnvalue_4))
  ;[1 1 1] Standard Raycast
  (if (Variables|/Game/Blueprints/BP_CB_Raycast_Component_00.BP_CB_Raycast_Component_00_C|GetSetObjectActive (Variables|Default|GetBP_CB_Activatable_Component_00))
    (bind _outhit (Collision|LineTraceByChannel _returnvalue _returnvalue_5 "TraceTypeQuery1" false 0 "None" true "(R=1.000000,G=0.000000,B=0.000000,A=1.000000)" "(R=0.000000,G=0.016063,B=1.000000,A=1.000000)" 0.1))
    (Class|ParticleSystemComponent|SetBeamTargetPoint _ps_lw_laserbeam_00 0 (.ImpactPoint (Collision|BreakHitResult _outhit)))
    (Effects|Components|ParticleSystem|SetEmitterEnable _ps_lw_laserbeam_00 "Beam" true)
    (Effects|Components|ParticleSystem|SetEmitterEnable _ps_lw_laserbeam_00 "BeamDischarge" true)
    (if (Actor|ActorHasTag (.HitActor (Collision|BreakHitResult _outhit)) "LaserActivatable")
      (Default|Active (Actor|GetComponentbyClass (.HitActor (Collision|BreakHitResult _outhit)) "/Game/Blueprints/BP_CB_Raycast_Component_00.BP_CB_Raycast_Component_00_C") (Variables|Laser|GetLaserColour))
      (Variables|Default|SetHasBeenActive true))
    ;[1 1 1] Reflection
    (if (or (Actor|ActorHasTag (.HitActor (Collision|BreakHitResult _outhit)) "Reflective") (Components|ComponentHasTag (.HitComponent (Collision|BreakHitResult _outhit)) "Reflective"))
      (bind _outhit_2 (Collision|LineTraceByChannel (+ (.ImpactPoint (Collision|BreakHitResult _outhit)) (.Normal (Collision|BreakHitResult _outhit))) (+ (.ImpactPoint (Collision|BreakHitResult _outhit)) (Math|Vector|MirrorVectorbyNormal (- _returnvalue_5 _returnvalue) (.ImpactNormal (Collision|BreakHitResult _outhit)))) "TraceTypeQuery1" false 0 "ForDuration" true "(R=1.000000,G=0.000000,B=0.000000,A=1.000000)" "(R=0.000000,G=0.039124,B=1.000000,A=1.000000)" 0.1))
      (if (Actor|ActorHasTag (.HitActor (Collision|BreakHitResult _outhit_2)) "LaserActivatable")
        (Default|Active (Actor|GetComponentbyClass (.HitActor (Collision|BreakHitResult _outhit_2)) "/Game/Blueprints/BP_CB_Raycast_Component_00.BP_CB_Raycast_Component_00_C") (Variables|Laser|GetLaserColour))
        (Variables|Default|SetHasBeenActive true)))
    (else
      (if (Variables|Default|GetHasBeenActive)
        (Default|NotActive (Actor|GetComponentbyClass (.HitActor (Collision|BreakHitResult _outhit)) "/Game/Blueprints/BP_CB_Raycast_Component_00.BP_CB_Raycast_Component_00_C"))
        (Variables|Default|SetHasBeenActive false))
      (Effects|Components|ParticleSystem|SetEmitterEnable _ps_lw_laserbeam_00 "Beam" false)
      (Effects|Components|ParticleSystem|SetEmitterEnable _ps_lw_laserbeam_00 "BeamDischarge" false))))

(event EventBeginPlay
  (bind _ps_lw_laserbeam_00 (Variables|Default|GetPS_LW_LaserBeam_00))
  (Effects|Components|ParticleSystem|SetColorParameter _ps_lw_laserbeam_00 "BeamColour" (Variables|Laser|GetLaserColour))
  (Effects|Components|ParticleSystem|SetEmitterEnable _ps_lw_laserbeam_00 "Beam" false)
  (Effects|Components|ParticleSystem|SetEmitterEnable _ps_lw_laserbeam_00 "BeamDischarge" false))

(fn ConstructionScript)

(fn NewFunction0
  (params (A :type Vector) (B :type Vector) (A2 :type Vector) (A3 :type Vector) (B2 :type Vector) (self2 :type Actor%20Object%20Reference) (InputPin :type Vector))
  (if (Actor|ActorHasTag self2 "Reflective")
    (bind _outhit (Collision|LineTraceByChannel (+ A3 B2) (+ A2 (Math|Vector|MirrorVectorbyNormal (- A B) InputPin)) "TraceTypeQuery1" false 0 "ForDuration" true "(R=1.000000,G=0.000000,B=0.000000,A=1.000000)" "(R=0.000000,G=0.039124,B=1.000000,A=1.000000)" 0.1))))