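; BP_CB_Charger_00 is a charger that adds a set amount to the player's power cell charge when activated.
; Tick polls the raycast component's active flag and clears it after a minimal delay.
; If the player has the power ball, a DoOnce applies the charge, so it works only once.
; BeginPlay caches the player by casting the player pawn to BP_CB_PlayerController_00.
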(event EventTick
  (params (DeltaSeconds :type Float%20%28single-precision%29))
  (bind _player (Variables|Default|GetPlayer))
  ;[1 1 1] Increments the Power cell charge when activated
  (if (Variables|/Game/Blueprints/UnicornCube/BP_CB_Raycast_Component_00.BP_CB_Raycast_Component_00_C|GetSetObjectActive (Variables|Default|GetBP_CB_Raycast_Component_00))
    (Utilities|FlowControl|Delay 0.0001)
    (Variables|/Game/Blueprints/UnicornCube/BP_CB_Raycast_Component_00.BP_CB_Raycast_Component_00_C|SetSetObjectActive (Variables|Default|GetBP_CB_Raycast_Component_00) false)
    (if (Variables|/Game/Blueprints/Player/BP_CB_PlayerController_00.BP_CB_PlayerController_00_C|GethasPowerBall _player)
      (Utilities|FlowControl|DoOnce false
        (:Completed
          (Variables|/Game/Blueprints/Player/BP_CB_PlayerController_00.BP_CB_PlayerController_00_C|SetPowerCellCharge _player (+ (Variables|/Game/Blueprints/Player/BP_CB_PlayerController_00.BP_CB_PlayerController_00_C|GetPowerCellCharge _player) (Variables|Default|GetChargeAmount))))))))

(event EventBeginPlay
  ;[1 1 1] Get Player
  (bind _asbp_cb_player_controller_00 (Utilities|Casting|CastToBP_CB_PlayerController_00 (Game|Player|GetPlayerPawn 0)))
  (Variables|Default|SetPlayer _asbp_cb_player_controller_00))

(fn ConstructionScript)