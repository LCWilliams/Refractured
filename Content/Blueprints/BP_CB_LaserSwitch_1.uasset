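; Laser receiver switch that becomes active when the incoming laser matches its required colour, within a tolerance, and its exact required power.
; Tick derives IsActive from the raycast component's active flag, sent colour and sent power.
; Paired DoOnce gates limit visual updates to changes between success and waiting states.
; A dynamic receiver-plate material, created in the construction script, displays the required colour and changes status colour, spin and pulse per state.
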(event EventTick
  (params (DeltaSeconds :type Float%20%28single-precision%29))
  (bind _bp_cb_raycast_component_00 (Variables|Default|GetBP_CB_Raycast_Component_00))
  ;[1 1 1] Sets Active if compared colour are close to equal
  (bind _output_get (Variables|Default|SetisActive (Math|Boolean|ANDBoolean (Variables|/Game/Blueprints/UnicornCube/BP_CB_Raycast_Component_00.BP_CB_Raycast_Component_00_C|GetSetObjectActive _bp_cb_raycast_component_00) (CallFunction|CompareColours (Variables|/Game/Blueprints/UnicornCube/BP_CB_Raycast_Component_00.BP_CB_Raycast_Component_00_C|GetSentColour _bp_cb_raycast_component_00) (Variables|Default|GetColourErrorTolerance) (Variables|Default|GetReqColour)) (== (Variables|/Game/Blueprints/UnicornCube/BP_CB_Raycast_Component_00.BP_CB_Raycast_Component_00_C|GetSentPower _bp_cb_raycast_component_00) (Variables|Default|GetRequiredPower)))))
  (if _output_get
    (Utilities|FlowControl|DoOnce false :!label _label
      (:Completed
        (CallFunction|ApplySuccess)
        (goto _label_2 Reset)))
    (else
      (Utilities|FlowControl|DoOnce true :!label _label_2
        (:Completed
          (CallFunction|ApplyWaiting)
          (goto _label Reset))))))

(fn ConstructionScript
  (bind _receiver (Variables|Default|GetReceiver))
  ;[1 1 1] Sets Switch Colour
  (|CallParentFunction)
  (bind _returnvalue (Rendering|Material|CreateDynamicMaterialInstance _receiver 1 "/Game/Materials/Other/M_LW_ReceiverPlate_00.M_LW_ReceiverPlate_00" :!class /Script/Engine.PrimitiveComponent))
  (bind _output_get (Variables|Default|SetDynamicMaterial _returnvalue))
  (Rendering|Material|SetMaterial _receiver 1 _returnvalue)
  (Rendering|Material|SetVectorParameterValue _output_get "InputColour" (Variables|Default|GetReqColour) :!class /Script/Engine.MaterialInstanceDynamic)
  (CallFunction|ApplyWaiting))

(fn ApplyWaiting
  (bind _dynamicmaterial (Variables|Default|GetDynamicMaterial))
  (Rendering|Material|SetVectorParameterValue _dynamicmaterial "InputColour" (Variables|Default|GetReqColour) :!class /Script/Engine.MaterialInstanceDynamic)
  (Rendering|Material|SetVectorParameterValue _dynamicmaterial "StatusColour" "(R=0.050000,G=0.050000,B=0.050000,A=1.000000)" :!class /Script/Engine.MaterialInstanceDynamic)
  (Rendering|Material|SetScalarParameterValue _dynamicmaterial "StatusSpinSpeed" 0.0 :!class /Script/Engine.MaterialInstanceDynamic)
  (Rendering|Material|SetScalarParameterValue _dynamicmaterial "ColourSpinSpeed" 0.0 :!class /Script/Engine.MaterialInstanceDynamic)
  (Rendering|Material|SetScalarParameterValue _dynamicmaterial "ColourPulseSpeed" 2.0 :!class /Script/Engine.MaterialInstanceDynamic))

(fn ApplySuccess
  (bind _dynamicmaterial (Variables|Default|GetDynamicMaterial))
  (Rendering|Material|SetVectorParameterValue _dynamicmaterial "StatusColour" "(R=0.000000,G=0.500000,B=0.500000,A=1.000000)" :!class /Script/Engine.MaterialInstanceDynamic)
  (Rendering|Material|SetScalarParameterValue _dynamicmaterial "StatusSpinSpeed" 25.0 :!class /Script/Engine.MaterialInstanceDynamic)
  (Rendering|Material|SetScalarParameterValue _dynamicmaterial "ColourSpinSpeed" 5.0 :!class /Script/Engine.MaterialInstanceDynamic)
  (Rendering|Material|SetScalarParameterValue _dynamicmaterial "ColourPulseSpeed" 0.0 :!class /Script/Engine.MaterialInstanceDynamic))