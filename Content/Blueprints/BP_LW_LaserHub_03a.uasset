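; Laser hub actor that fires a beam from a mesh socket and activates objects it hits.
; Every Tick it line-traces forward, ends the particle beam at the impact and passes LaserColour to the raycast component of LaserActivatable actors.
; Reflective hits trigger one mirrored trace that can also activate targets but shows only as a debug line.
; Switch-off and beam-colour logic are disconnected, and CastLaser and LaserBounce are unfinished stubs.
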(event Collision|EventActorBeginOverlap
  (params (OtherActor :type Actor%20Object%20Reference)))

(event EventTick
  (params (DeltaSeconds :type Float%20%28single-precision%29))
  (bind _ps_lw_laserbeam_00 (Variables|Default|GetPS_LW_LaserBeam_00))
  (bind _skm_lw_laser_00_laser (Variables|Default|GetSkM_LW_Laser_00_Laser))
  (bind _returnvalue (Transformation|GetSocketTransform _skm_lw_laser_00_laser "Socket_LaserOrigin" "RTS_Actor"))
  (bind _returnvalue_2 (Math|Vector|GetForwardVector (.rotation _returnvalue)))
  (bind _returnvalue_3 (* _returnvalue_2 1e+04))
  (bind _returnvalue_4 (+ (.location _returnvalue) _returnvalue_3))
  ;[1 1 1] Standard Raycast
  (bind _outhit (Collision|LineTraceByChannel (.location _returnvalue) _returnvalue_4 "TraceTypeQuery1" false 0 "None" true "(R=1.000000,G=0.000000,B=0.000000,A=1.000000)" "(R=0.000000,G=0.016063,B=1.000000,A=1.000000)" 0.1))
  (Class|ParticleSystemComponent|SetBeamTargetPoint _ps_lw_laserbeam_00 0 (.ImpactPoint (Collision|BreakHitResult _outhit)))
  (Effects|Components|ParticleSystem|SetEmitterEnable _ps_lw_laserbeam_00 "Beam" true)
  (Effects|Components|ParticleSystem|SetEmitterEnable _ps_lw_laserbeam_00 "BeamDischarge" true)
  (if (Actor|ActorHasTag (.HitActor (Collision|BreakHitResult _outhit)) "LaserActivatable")
    (Default|Active (Actor|GetComponentbyClass (.HitActor (Collision|BreakHitResult _outhit)) "/Game/Blueprints/BP_CB_Raycast_Component_00.BP_CB_Raycast_Component_00_C") (Variables|Default|GetLaserColour))
    (Variables|Default|SetHas%20Been%20Active true))
  ;[1 1 1] Reflection
  (if (or (Actor|ActorHasTag (.HitActor (Collision|BreakHitResult _outhit)) "Reflective") (Components|ComponentHasTag (.HitComponent (Collision|BreakHitResult _outhit)) "Reflective"))
    (bind _outhit_2 (Collision|LineTraceByChannel (+ (.ImpactPoint (Collision|BreakHitResult _outhit)) (.Normal (Collision|BreakHitResult _outhit))) (+ (.ImpactPoint (Collision|BreakHitResult _outhit)) (Math|Vector|MirrorVectorbyNormal (- _returnvalue_4 (.location _returnvalue)) (.ImpactNormal (Collision|BreakHitResult _outhit)))) "TraceTypeQuery1" false 0 "ForDuration" true "(R=1.000000,G=0.000000,B=0.000000,A=1.000000)" "(R=0.000000,G=0.039124,B=1.000000,A=1.000000)" 0.1))
    (if (Actor|ActorHasTag (.HitActor (Collision|BreakHitResult _outhit_2)) "LaserActivatable")
      (Default|Active (Actor|GetComponentbyClass (.HitActor (Collision|BreakHitResult _outhit_2)) "/Game/Blueprints/BP_CB_Raycast_Component_00.BP_CB_Raycast_Component_00_C") (Variables|Default|GetLaserColour))
      (Variables|Default|SetHas%20Been%20Active true))))

(event EventBeginPlay
  (bind _ps_lw_laserbeam_00 (Variables|Default|GetPS_LW_LaserBeam_00))
  (bind _skm_lw_laser_00_laser (Variables|Default|GetSkM_LW_Laser_00_Laser))
  (bind _returnvalue (Transformation|GetSocketTransform _skm_lw_laser_00_laser "Socket_LaserOrigin" "RTS_Actor"))
  (bind _returnvalue_2 (Math|Vector|GetForwardVector (.rotation _returnvalue)))
  (bind _returnvalue_3 (* _returnvalue_2 1e+04))
  (bind _returnvalue_4 (+ (.location _returnvalue) _returnvalue_3))
  (Class|ParticleSystemComponent|SetBeamSourcePoint _ps_lw_laserbeam_00 0 (.location _returnvalue))
  ;[1 1 1] Standard Raycast
  (bind _outhit (Collision|LineTraceByChannel (.location _returnvalue) _returnvalue_4 "TraceTypeQuery1" false 0 "None" true "(R=1.000000,G=0.000000,B=0.000000,A=1.000000)" "(R=0.000000,G=0.016063,B=1.000000,A=1.000000)" 0.1))
  (Class|ParticleSystemComponent|SetBeamTargetPoint _ps_lw_laserbeam_00 0 (.ImpactPoint (Collision|BreakHitResult _outhit)))
  (Effects|Components|ParticleSystem|SetEmitterEnable _ps_lw_laserbeam_00 "Beam" true)
  (Effects|Components|ParticleSystem|SetEmitterEnable _ps_lw_laserbeam_00 "BeamDischarge" true)
  (if (Actor|ActorHasTag (.HitActor (Collision|BreakHitResult _outhit)) "LaserActivatable")
    (Default|Active (Actor|GetComponentbyClass (.HitActor (Collision|BreakHitResult _outhit)) "/Game/Blueprints/BP_CB_Raycast_Component_00.BP_CB_Raycast_Component_00_C") (Variables|Default|GetLaserColour))
    (Variables|Default|SetHas%20Been%20Active true))
  ;[1 1 1] Reflection
  (if (or (Actor|ActorHasTag (.HitActor (Collision|BreakHitResult _outhit)) "Reflective") (Components|ComponentHasTag (.HitComponent (Collision|BreakHitResult _outhit)) "Reflective"))
    (bind _outhit_2 (Collision|LineTraceByChannel (+ (.ImpactPoint (Collision|BreakHitResult _outhit)) (.Normal (Collision|BreakHitResult _outhit))) (+ (.ImpactPoint (Collision|BreakHitResult _outhit)) (Math|Vector|MirrorVectorbyNormal (- _returnvalue_4 (.location _returnvalue)) (.ImpactNormal (Collision|BreakHitResult _outhit)))) "TraceTypeQuery1" false 0 "ForDuration" true "(R=1.000000,G=0.000000,B=0.000000,A=1.000000)" "(R=0.000000,G=0.039124,B=1.000000,A=1.000000)" 0.1))
    (if (Actor|ActorHasTag (.HitActor (Collision|BreakHitResult _outhit_2)) "LaserActivatable")
      (Default|Active (Actor|GetComponentbyClass (.HitActor (Collision|BreakHitResult _outhit_2)) "/Game/Blueprints/BP_CB_Raycast_Component_00.BP_CB_Raycast_Component_00_C") (Variables|Default|GetLaserColour))
      (Variables|Default|SetHas%20Been%20Active true))))

(fn ConstructionScript)

(fn CastLaser)