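; BP_LW_Door_3x5_01 is a sliding door that opens while all its referenced laser receivers are active.
; A looping timeline, rate-scaled by PerformanceDelay, polls ReceiverChecker on an event track instead of using Tick.
; ReceiverChecker counts active receivers only when RequiresPower is set, resetting on any inactive one.
; The result plays or reverses DoorTimeLine, which moves four mesh pieces along one vector track, one offset in X.
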(event EventBeginPlay
  (Components|Timeline|SetPlayRate (Variables|Default|GetLooping) (Variables|Optimization|GetPerformanceDelay))
  (Timeline|Looping PlayFromStart
    (:NewTrack_1
      (bind _returnvalue (CallFunction|ReceiverChecker))
      (if _returnvalue
        (bind _door1 (Timeline|DoorTimeLine Play)
          (:Update
            (Transformation|SetRelativeLocation (Variables|Default|GetSM_LW_Door_3x5_01_b) (Math|Vector|MakeVector (- (.X (Math|Vector|BreakVector _door1)) 1e+01) (.Y (Math|Vector|BreakVector _door1)) (.Z (Math|Vector|BreakVector _door1))) false false)
            (Transformation|SetRelativeLocation (Variables|Default|GetSM_LW_Door_3x5_01_c) _door1 false false)))
        (else
          (Variables|Default|SetActivated 0)
          (Timeline|DoorTimeLine Reverse))))))

(fn ConstructionScript)

(fn ReceiverChecker
  (bind _laserrecieverref (Variables|Configuration|GetLaserRecieverRef))
  (if (Variables|Configuration|GetRequiresPower)
    (Variables|Default|SetActivated 0)
    (for _array_element _laserrecieverref
      (if (Variables|/Game/Blueprints/Parents/BP_CB_ParentDontUse_00.BP_CB_ParentDontUse_00_C|GetisActive _array_element)
        (bind _result (Math|Integer|IncrementInt (Variables|Default|GetActivated))
          (:%20%20
            (Variables|Default|SetActivated _result)))
        (else
          (Variables|Default|SetActivated 0))))
    (return (>= (Variables|Default|GetActivated) (Utilities|Array|Length _laserrecieverref)))))