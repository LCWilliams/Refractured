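; Laser puzzle cube whose six faces are each set to reflect, take input, refract out or disperse out.
; The construction script assigns face meshes and creates a laser particle pool for each output face.
; While hit, Tick adds incoming colour to the held colour, then fires outputs: refract in that colour, dispersion in its face colour if the held RGB covers it.
; A DoOnce clears colour, power and lasers when the hit ends.
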(event EventTick
  (params (DeltaSeconds :type Float%20%28single-precision%29))
  (if (Variables|Default|GetHit)
    (Utilities|FlowControl|Sequence
      (:then_0
        (if (Variables|/Game/Blueprints/UnicornCube/BP_CB_Raycast_Component_00.BP_CB_Raycast_Component_00_C|GetSetObjectActive (Variables|Default|GetBP_CB_Raycast_Component_00))
          (Variables|Default|SetHit true)
          (else
            (Variables|Default|SetHit false))))
      (:then_1
        (Utilities|UpdateReceived
          (:Out
            (Utilities|UpdateFaces))))
      (:then_2
        (goto _label Reset)))
    (else
      (Utilities|FlowControl|DoOnce false :!label _label
        (:Completed
          (Utilities|DisableLasers))))))

(fn ConstructionScript
  (Setup|CreateFaces))

(fn CreateFaces
  (bind _output_get (Variables|Settings|SetFaces (Utilities|Array|MakeArray (Variables|Default|GetFace_Front) (Variables|Default|GetFace_Back) (Variables|Default|GetFace_Left) (Variables|Default|GetFace_Right) (Variables|Default|GetFace_Top) (Variables|Default|GetFace_Bottom))))
  (Variables|Settings|SetLaserComponents (Utilities|Array|MakeArray (Variables|Component:LaserComponent|GetLaserComponent_Front) (Variables|Component:LaserComponent|GetLaserComponent_Back) (Variables|Component:LaserComponent|GetLaserComponent_Left) (Variables|Component:LaserComponent|GetLaserComponent_Right) (Variables|Component:LaserComponent|GetLaserComponent_Top) (Variables|Component:LaserComponent|GetLaserComponent_Bottom)))
  (bind _output_get_2 (Variables|Settings|SetFaceSettings (Utilities|Array|MakeArray (Variables|Settings|GetFront) (Variables|Settings|GetBack) (Variables|Settings|GetLeft) (Variables|Settings|GetRight) (Variables|Settings|GetTop) (Variables|Settings|GetBottom))))
  (for (_array_element _array_index) _output_get_2
    (switch Utilities|FlowControl|Switch|SwitchonE_LW_Cube_01 _array_element
      (:NewEnumerator4
        (Components|StaticMesh|SetStaticMesh (Utilities|Array|Get(acopy) _output_get _array_index) (Variables|Settings|GetReflectionFace)))
      (:NewEnumerator1
        (Components|StaticMesh|SetStaticMesh (Utilities|Array|Get(acopy) _output_get _array_index) (Variables|Settings|GetInputFace)))
      (:NewEnumerator2
        (Components|StaticMesh|SetStaticMesh (Utilities|Array|Get(acopy) _output_get _array_index) (Variables|Settings|GetOutputFace))
        (bind _laserparticlearray (CallFunction|InstantiateLasers (Variables|PassThroughVariables|GetMaxBounce) (Variables|Settings|GetLaser%20Particle%20Template) false (Transformation|GetActorLocation self) :!label _label))
        (Setup|AddLaserstoFace _array_index _laserparticlearray))
      (:NewEnumerator3
        (Components|StaticMesh|SetStaticMesh (Utilities|Array|Get(acopy) _output_get _array_index) (Variables|Settings|GetOutputFace))
        (CallFunction|MakeDispersionSettings _array_index)
        (goto _label)))))

(fn AddLaserstoFace
  (params (Loop%20Index :type Integer) (Particles%20To%20Add :type Array%20of%20Particle%20System%20Component%20Object%20References))
  (switch int Loop%20Index
    (:0
      (Variables|FaceParticles|SetLasers_Front Particles%20To%20Add))
    (:1
      (Variables|FaceParticles|SetLasers_Back Particles%20To%20Add))
    (:2
      (Variables|FaceParticles|SetLasers_Left Particles%20To%20Add))
    (:3
      (Variables|FaceParticles|SetLasers_Right Particles%20To%20Add))
    (:4
      (Variables|FaceParticles|SetLasers_Top Particles%20To%20Add))
    (:5
      (Variables|FaceParticles|SetLasers_Bottom Particles%20To%20Add)))
  (return))

(fn MakeDispersionSettings
  (params (FaceIndex :type Integer)))

(fn RefractS
  (params (Array%20Index :type Integer%20%28by%20ref%29))
  (bind _faces (Variables|Settings|GetFaces))
  (bind _lasercomponents (Variables|Settings|GetLaserComponents))
  (bind _item (Utilities|Array|Get(acopy) _faces Array%20Index))
  (bind _item_2 (Utilities|Array|Get(acopy) _lasercomponents Array%20Index))
  (switch int Array%20Index
    (:0
      (Default|FireLaser _item_2 _item (Variables|Default|GetHeldColour) (Variables|FaceParticles|GetLasers_Front) (Variables|PassThroughVariables|GetMaxBounce) (Variables|PassThroughVariables|GetInputPower)))
    (:1
      (Default|FireLaser _item_2 _item (Variables|Default|GetHeldColour) (Variables|FaceParticles|GetLasers_Back) (Variables|PassThroughVariables|GetMaxBounce) (Variables|PassThroughVariables|GetInputPower)))
    (:2
      (Default|FireLaser _item_2 _item (Variables|Default|GetHeldColour) (Variables|FaceParticles|GetLasers_Left) (Variables|PassThroughVariables|GetMaxBounce) (Variables|PassThroughVariables|GetInputPower)))
    (:3
      (Default|FireLaser _item_2 _item (Variables|Default|GetHeldColour) (Variables|FaceParticles|GetLasers_Right) (Variables|PassThroughVariables|GetMaxBounce) (Variables|PassThroughVariables|GetInputPower)))
    (:4
      (Default|FireLaser _item_2 _item (Variables|Default|GetHeldColour) (Variables|FaceParticles|GetLasers_Top) (Variables|PassThroughVariables|GetMaxBounce) (Variables|PassThroughVariables|GetInputPower)))
    (:5
      (Default|FireLaser _item_2 _item (Variables|Default|GetHeldColour) (Variables|FaceParticles|GetLasers_Bottom) (Variables|PassThroughVariables|GetMaxBounce) (Variables|PassThroughVariables|GetInputPower)))))

(fn RefractD
  (params (Array%20Index :type Integer%20%28by%20ref%29))
  (bind _faces (Variables|Settings|GetFaces))
  (bind _lasercomponents (Variables|Settings|GetLaserComponents))
  (bind _frontdispersion (Variables|DispersionValues|GetFrontDispersion))
  (bind _backdispersion (Variables|DispersionValues|GetBackDispersion))
  (bind _leftdispersion (Variables|DispersionValues|GetLeftDispersion))
  (bind _rightdispersion (Variables|DispersionValues|GetRightDispersion))
  (bind _topdispersion (Variables|DispersionValues|GetTopDispersion))
  (bind _bottomdispersion (Variables|DispersionValues|GetBottomDispersion))
  (bind _item (Utilities|Array|Get(acopy) _faces Array%20Index))
  (bind _item_2 (Utilities|Array|Get(acopy) _lasercomponents Array%20Index))
  (switch int Array%20Index
    (:0
      (if (Check|DispersionCheck _frontdispersion)
        (Default|FireLaser _item_2 _item _frontdispersion (Variables|FaceParticles|GetLasers_Front) (Variables|PassThroughVariables|GetMaxBounce) (Variables|PassThroughVariables|GetInputPower))))
    (:1
      (if (Check|DispersionCheck _backdispersion)
        (Default|FireLaser _item_2 _item _backdispersion (Variables|FaceParticles|GetLasers_Back) (Variables|PassThroughVariables|GetMaxBounce) (Variables|PassThroughVariables|GetInputPower))))
    (:2
      (if (Check|DispersionCheck _leftdispersion)
        (Default|FireLaser _item_2 _item _leftdispersion (Variables|FaceParticles|GetLasers_Left) (Variables|PassThroughVariables|GetMaxBounce) (Variables|PassThroughVariables|GetInputPower))))
    (:3
      (if (Check|DispersionCheck _rightdispersion)
        (Default|FireLaser _item_2 _item _rightdispersion (Variables|FaceParticles|GetLasers_Right) (Variables|PassThroughVariables|GetMaxBounce) (Variables|PassThroughVariables|GetInputPower))))
    (:4
      (if (Check|DispersionCheck _topdispersion)
        (Default|FireLaser _item_2 _item _topdispersion (Variables|FaceParticles|GetLasers_Top) (Variables|PassThroughVariables|GetMaxBounce) (Variables|PassThroughVariables|GetInputPower))))
    (:5
      (if (Check|DispersionCheck _bottomdispersion)
        (Default|FireLaser _item_2 _item _bottomdispersion (Variables|FaceParticles|GetLasers_Bottom) (Variables|PassThroughVariables|GetMaxBounce) (Variables|PassThroughVariables|GetInputPower))))))

(fn DispersionCheck
  (params (DispersionColour :type Linear%20Color%20Structure%20%28by%20ref%29))
  (bind _heldcolour (Variables|Default|GetHeldColour))
  (return (Math|Boolean|ANDBoolean (>= (.r _heldcolour) (.r DispersionColour)) (>= (.g _heldcolour) (.g DispersionColour)) (>= (.b _heldcolour) (.b DispersionColour)))))