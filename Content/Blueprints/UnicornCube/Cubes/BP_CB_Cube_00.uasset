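; Laser puzzle cube that receives a beam and re-emits it in the same colour from its output or refraction faces.
; BeginPlay builds parallel arrays of six laser components, direction arrows and beam visuals, indexed by face.
; Each tick it walks the face-type array: input faces set the hit state from a single raycast component.
; While hit, emitting faces fire along their arrows with a bounce limit and show their beams, otherwise the beams are deactivated.
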(event EventBeginPlay
  (CallFunction|MakeArrays))

(event EventTick
  (params (DeltaSeconds :type Float%20%28single-precision%29))
  (Utilities|UpdateFaces))

(fn ConstructionScript)

(fn MakeArrays
  (Variables|Faces|SetFaceLasers (Utilities|Array|MakeArray (Variables|Default|GetBP_CB_Laser_Component_00) (Variables|Default|GetBP_CB_Laser_Component_01) (Variables|Default|GetBP_CB_Laser_Component_02) (Variables|Default|GetBP_CB_Laser_Component_03) (Variables|Default|GetBP_CB_Laser_Component_04) (Variables|Default|GetBP_CB_Laser_Component_05)))
  (Variables|Faces|SetArrows (Utilities|Array|MakeArray (Variables|Default|GetArrow) (Variables|Default|GetArrow1) (Variables|Default|GetArrow2) (Variables|Default|GetArrow3) (Variables|Default|GetArrow4) (Variables|Default|GetArrow5)))
  (Variables|Faces|SetVisualLasers (Utilities|Array|MakeArray (Variables|Default|GetPS_LW_LaserBeam_00) (Variables|Default|GetPS_LW_LaserBeam_01) (Variables|Default|GetPS_LW_LaserBeam_02) (Variables|Default|GetPS_LW_LaserBeam_03) (Variables|Default|GetPS_LW_LaserBeam_04) (Variables|Default|GetPS_LW_LaserBeam_05))))