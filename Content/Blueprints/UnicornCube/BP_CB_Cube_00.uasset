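; Puzzle cube with six configurable faces that receives a laser and re-emits it as refracted or colour-dispersed beams.
; Each tick, the raycast component supplies hit state, colour and power, and each face acts by its enum role.
; Refraction fires that face's laser component and toggles its beam visual.
; Dispersion first isolates red, green or blue above a tolerance; the construction script pre-sizes splines for bounces.
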(event EventBeginPlay
  (CallFunction|MakeArrays))

(event EventTick
  (params (DeltaSeconds :type Float%20%28single-precision%29))
  (Utilities|UpdateFaces))

(fn ConstructionScript
  (bind _tangents (LocalVariables|GetTangents))
  (bind _tangents_2 (LocalVariables|GetTangents))
  (for _array_element (Variables|Faces|GetSplineArrays)
    (Spline|SetTangentsatSplinePoint _array_element 1 _tangents_2 _tangents_2 "Local" true)
    (for _index (range 0 (- (Variables|Default|GetMaxBounce) 2))
      (Spline|AddSplinePoint _array_element (LocalVariables|GetPosition) "Local" true)
      (Spline|SetTangentsatSplinePoint _array_element _index _tangents _tangents "Local" true))))

(fn MakeArrays
  (Variables|Faces|SetFaceLasers (Utilities|Array|MakeArray (Variables|Default|GetBP_CB_Laser_Component_00) (Variables|Default|GetBP_CB_Laser_Component_01) (Variables|Default|GetBP_CB_Laser_Component_02) (Variables|Default|GetBP_CB_Laser_Component_03) (Variables|Default|GetBP_CB_Laser_Component_04) (Variables|Default|GetBP_CB_Laser_Component_05)))
  (Variables|Faces|SetArrows (Utilities|Array|MakeArray (Variables|Default|GetArrow) (Variables|Default|GetArrow1) (Variables|Default|GetArrow2) (Variables|Default|GetArrow3) (Variables|Default|GetArrow4) (Variables|Default|GetArrow5)))
  (Variables|Faces|SetVisualLasers (Utilities|Array|MakeArray (Variables|Default|GetPS_LW_LaserBeam_00) (Variables|Default|GetPS_LW_LaserBeam_01) (Variables|Default|GetPS_LW_LaserBeam_02) (Variables|Default|GetPS_LW_LaserBeam_03) (Variables|Default|GetPS_LW_LaserBeam_04) (Variables|Default|GetPS_LW_LaserBeam_05)))
  (Variables|Faces|SetSplineArrays (Utilities|Array|MakeArray (Variables|Default|GetSpline) (Variables|Default|GetSpline1) (Variables|Default|GetSpline2) (Variables|Default|GetSpline3) (Variables|Default|GetSpline4) (Variables|Default|GetSpline5))))