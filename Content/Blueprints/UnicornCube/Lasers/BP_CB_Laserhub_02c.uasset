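; Possessable laser emitter pawn that the player aims by rotating the body and head bones of its skeletal mesh, with clamped pitch.
; When flagged active, it hands possession over through the player controller pawn, and the Activate input returns control.
; A looping timeline stands in for Tick, syncing the socket-attached arrow and camera and firing a bouncing, coloured beam through the laser component.
; If it needs power, it fires only when its linked receivers are active.
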(event EventTick
  (params (DeltaSeconds :type Float%20%28single-precision%29))
  ;[1 1 1] Laser Pawn Possession
  (bind _bp_cb_raycast_component_00 (PlayerControl|Possession)))

(event EventBeginPlay
  (bind _skm_lw_laser_01_laserbase (Variables|Default|GetSkM_LW_Laser_01_LaserBase))
  (bind _bp_cb_laser_component_01 (Variables|Default|GetBP_CB_Laser_Component_01))
  (bind _ps_lw_laserbeam_00 (Variables|Default|GetPS_LW_LaserBeam_00))
  ;[1 1 1] Initialise Components
  (Utilities|FlowControl|Sequence
    (:then_0
      (Transformation|AttachComponentToComponent (Variables|Default|GetArrow) _skm_lw_laser_01_laserbase "Socket_LaserOrigin" "SnapToTarget" "SnapToTarget" "SnapToTarget" false)
      (Transformation|AttachComponentToComponent (Variables|Default|GetCamera) _skm_lw_laser_01_laserbase "Socket_LaserCamera" "SnapToTarget" "SnapToTarget" "SnapToTarget" false)
      (Components|Activation|SetActive _ps_lw_laserbeam_00 false false)
      (Default|TraceSetup _bp_cb_laser_component_01 (Variables|Default|GetArrow)))
    (:then_1
      ;[1 1 1] Event Tick Replacer
      (Components|Timeline|SetPlayRate (Variables|Default|GetLooping) (Variables|Default|GetPerformanceDelay))
      (Timeline|Looping PlayFromStart
        (:NewTrack_1
          ;[1 1 1] Raycast
          (Adjustments|CameraLaserRotation)
          (if (Variables|Activation|GetNeedsPower)
            (bind _recievers (CallFunction|ReciverChecker))
            (if _recievers
              (Default|FireLaser _bp_cb_laser_component_01 (Variables|Default|GetArrow) (Variables|Laser|GetLaserColour) (Variables|Default|GetPS_LW_LaserBeam_00) (Variables|Default|GetMaxBounce) :!label _label)
              (else
                (Components|Activation|SetActive _ps_lw_laserbeam_00 false false)))
            (else
              (goto _label))))))))

(event Input|ActionEvents|InputActionActivate
  (params (Key :type Key%20Structure :default "AnyKey"))
  (bind _returnvalue (Game|GetPlayerController 0))
  ;[1 1 1] Laser Pawn Possession
  (:Pressed
    (Variables|/Game/Blueprints/UnicornCube/BP_CB_Raycast_Component_00.BP_CB_Raycast_Component_00_C|SetSetObjectActive (stale EventTick _bp_cb_raycast_component_00) false)
    (Pawn|UnPossess _returnvalue)
    (Pawn|Possess _returnvalue (Variables|Default|GetPlayer%20Controller))))

(event Input|AxisEvents|InputAxisTurn
  (params (AxisValue :type Float%20%28single-precision%29))
  ;[1 1 1] Laser Rotation
  (bind _output_get (PlayerControl|RotationYaw AxisValue (Variables|Rotation|GetZ-Speed) (Utilities|Time|GetWorldDeltaSeconds) (Variables|Default|GetSkM_LW_Laser_01_LaserBase))))

(event Input|AxisEvents|InputAxisLookUp
  (params (AxisValue :type Float%20%28single-precision%29))
  ;[1 1 1] Laser Rotation
  (PlayerControl|RotationPitch (stale Input|AxisEvents|InputAxisTurn _output_get) AxisValue (Variables|Rotation|GetX-Speed) (Utilities|Time|GetWorldDeltaSeconds) (Variables|Default|GetSkM_LW_Laser_01_LaserBase)))

(fn ConstructionScript)

(fn Possession
  (bind _bp_cb_raycast_component_00 (Variables|Default|GetBP_CB_Raycast_Component_00))
  (bind _setobjectactive (Variables|/Game/Blueprints/UnicornCube/BP_CB_Raycast_Component_00.BP_CB_Raycast_Component_00_C|GetSetObjectActive _bp_cb_raycast_component_00))
  (if _setobjectactive
    (bind _asbp_cb_player_controller_00 (Utilities|Casting|CastToBP_CB_PlayerController_00 (Game|Player|GetPlayerPawn 0))
      (:then
        (bind _output_get (Variables|Default|SetPlayer%20Controller _asbp_cb_player_controller_00))
        (Default|TogglePossesion _output_get _setobjectactive self))
      (:CastFailed
        _)))
  (return _bp_cb_raycast_component_00))

(fn RotationYaw
  (params (InputAxis :type Float%20%28single-precision%29) (RotationSpeedModifier :type Float%20%28single-precision%29) (DeltaSeconds :type Float%20%28single-precision%29) (SkelatalMesh :type Poseable%20Mesh%20Component%20Object%20Reference))
  (bind _output_get (Variables|Rotation|SetCurrent%20Yaw (+ (stale _output_get) (* InputAxis RotationSpeedModifier DeltaSeconds))))
  (Components|PoseableMesh|SetBoneRotationbyName SkelatalMesh "LaserBody" (Math|Rotator|MakeRotator 9e+01 0.0 _output_get) "ComponentSpace")
  (return _output_get))

(fn RotationPitch
  (params (RotationYaw :type Float%20%28single-precision%29) (InputAxis :type Float%20%28single-precision%29) (RotationSpeedModifier :type Float%20%28single-precision%29) (DeltaSeconds :type Float%20%28single-precision%29) (SkelatalMesh :type Poseable%20Mesh%20Component%20Object%20Reference))
  (bind _output_get (Variables|Rotation|SetCurrent%20Pitch (+ (stale _output_get) (* InputAxis RotationSpeedModifier DeltaSeconds -1.0))))
  (bind _output_get_2 (Variables|Rotation|SetCurrent%20Pitch (Math|Float|Clamp(Float) _output_get 1.5e+02 2.4e+02)))
  (Components|PoseableMesh|SetBoneRotationbyName SkelatalMesh "LaserHead" (Math|Rotator|MakeRotator _output_get_2 1.8e+02 RotationYaw) "ComponentSpace"))

(fn DivideRotator
  (params (InputRotation :type Rotator))
  (bind (_roll _pitch _yaw) (Math|Rotator|BreakRotator InputRotation))
  (bind _rotationcorector (LocalVariables|GetRotationCorector))
  (return (Math|Rotator|MakeRotator (/ _roll _rotationcorector) (/ _pitch _rotationcorector) (/ _yaw _rotationcorector))))

(fn CameraLaserRotation
  (bind _skm_lw_laser_01_laserbase (Variables|Default|GetSkM_LW_Laser_01_LaserBase))
  (Transformation|SetRelativeRotation (Variables|Default|GetArrow) (Adjustments|DivideRotator (Transformation|GetSocketRotation _skm_lw_laser_01_laserbase "Socket_LaserOrigin")) false false)
  (Transformation|SetRelativeRotation (Variables|Default|GetCamera) (Adjustments|DivideRotator (Transformation|GetSocketRotation _skm_lw_laser_01_laserbase "Socket_LaserCamera")) false false))

(fn ReciverChecker
  (bind _receiverref (Variables|Activation|GetReceiverRef))
  (Variables|Default|SetActivated 0)
  (for _array_element _receiverref
    (if (Variables|/Game/Blueprints/Parents/BP_CB_ParentDontUse_00.BP_CB_ParentDontUse_00_C|GetisActive _array_element)
      (bind _result (Math|Integer|IncrementInt (Variables|Default|GetActivated))
        (:%20%20
          (Variables|Default|SetActivated _result)))
      (else
        (Variables|Default|SetActivated 0))))
  (return (>= (Variables|Default|GetActivated) (Utilities|Array|Length _receiverref))))