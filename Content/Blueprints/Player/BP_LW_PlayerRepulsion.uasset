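; BP_LW_PlayerRepulsion is a short-lived effect actor that drives a repulsion visual tied to the player's position.
; On BeginPlay it plays its audio source and sets its lifespan from the Lifetime variable.
; Every tick it casts player pawn 0 to BP_CB_PlayerController_00 and writes that location into the RepulsionEffect component's PlayerLocation vector parameter.
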(event EventBeginPlay
  (Audio|Components|Audio|Play (Variables|Default|GetAudioSource) 0.0)
  (Actor|SetLifeSpan (Variables|Default|GetLifetime)))

(event EventTick
  (params (DeltaSeconds :type Float%20%28single-precision%29))
  (bind _output_get (Variables|Default|SetPlayer%20Location (Transformation|GetActorLocation (.AsBP%20CB%20Player%20Controller%2000 (Utilities|Casting|CastToBP_CB_PlayerController_00 (Game|Player|GetPlayerPawn 0))))))
  (Effects|Components|ParticleSystem|SetVectorParameter (Variables|Default|GetRepulsionEffect) "PlayerLocation" _output_get))

(fn ConstructionScript)