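; Moving platform Blueprint that travels between a start and end point when it needs power and its linked laser receivers are all active.
; A looping timeline, with its play rate set by PerformanceDelay, polls the receivers through an event track instead of using Tick.
; ReceiverChecker counts active receivers, and the result plays or reverses PlatformTimeLine, which lerps the mesh's relative location.
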(event EventBeginPlay
  (Components|Timeline|SetPlayRate (Variables|Default|GetLooping) (Variables|Default|GetPerformanceDelay))
  (Timeline|Looping PlayFromStart
    (:NewTrack_1
      (if (Variables|Default|GetNeedsPower)
        (bind _returnvalue (CallFunction|ReceiverChecker))
        (if _returnvalue
          (bind _platform (Timeline|PlatformTimeLine Play)
            (:Update
              (Transformation|SetRelativeLocation (Variables|Default|GetSM_MC_Platform_00) (Math|Vector|Lerp(Vector) (Variables|Default|GetStartPoint) (Variables|Default|GetEndPoint) _platform) false false)))
          (else
            (Variables|Default|SetActivated 0)
            (Timeline|PlatformTimeLine Reverse)))))))

(fn ConstructionScript)

(fn ReceiverChecker
  (bind _laserrecieverref (Variables|Default|GetLaserRecieverRef))
  (Variables|Default|SetActivated 0)
  (for _array_element _laserrecieverref
    (if (Variables|/Game/Blueprints/BP_CB_LaserReciever_00.BP_CB_LaserReciever_00_C|GetisActive _array_element)
      (bind _result (Math|Integer|IncrementInt (Variables|Default|GetActivated))
        (:%20%20
          (Variables|Default|SetActivated _result)))
      (else
        (Variables|Default|SetActivated 0))))
  (return (>= (Variables|Default|GetActivated) (Utilities|Array|Length _laserrecieverref))))