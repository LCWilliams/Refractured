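; Door Blueprint that opens two panels when its referenced laser receivers satisfy the power check.
; A timeline, with play rate set by PerformanceDelay, polls ReceiverChecker through its event track.
; The result plays or reverses DoorTimeLine, whose update slides and tilts the panels.
; ReceiverChecker compares an active count to the receiver total, but returns inside the loop, so only the first receiver gets evaluated.
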(event EventBeginPlay
  (Components|Timeline|SetPlayRate (Variables|Default|GetLooping) (Variables|Optimization|GetPerformanceDelay))
  (Timeline|Looping PlayFromStart
    (:NewTrack_1
      (bind _returnvalue (CallFunction|ReceiverChecker))
      (if _returnvalue
        (bind (_direction _door_roty _door_x _door_z) (Timeline|DoorTimeLine Play)
          (:Update
            (Transformation|SetRelativeLocationAndRotation (Variables|Default|GetSM_MC_Door_Panel1_00) (Math|Vector|MakeVector 0.0 0.0 _door_z) (Math|Rotator|MakeRotator 0.0 _door_roty 0.0) false false)
            (Transformation|SetRelativeLocationAndRotation (Variables|Default|GetSM_MC_Door_Panel0_00) (+ (Math|Vector|MakeVector _door_x 0.0 0.0) (Math|Vector|MakeVector 0.0 0.0 _door_z)) (Math|Rotator|MakeRotator 0.0 _door_roty 0.0) false false)))
        (else
          (Variables|Default|SetActivated 0)
          (Timeline|DoorTimeLine Reverse))))))

(fn ConstructionScript)

(fn ReceiverChecker
  (bind _laserrecieverref (Variables|Configuration|GetLaserRecieverRef))
  (if (Variables|Configuration|GetRequiresPower)
    (Variables|Default|SetActivated 0)
    (for _array_element _laserrecieverref
      (if (Variables|/Game/Blueprints/BP_CB_LaserReciever_00.BP_CB_LaserReciever_00_C|GetisActive _array_element)
        (bind _result (Math|Integer|IncrementInt (Variables|Default|GetActivated))
          (:%20%20
            (Variables|Default|SetActivated _result)))
        (else
          (Variables|Default|SetActivated 0)))
      (return (>= (Variables|Default|GetActivated) (Utilities|Array|Length _laserrecieverref)))))
  (return (>= (Variables|Default|GetActivated) (Utilities|Array|Length _laserrecieverref))))