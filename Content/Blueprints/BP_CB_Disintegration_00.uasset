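; Decontamination chamber with a switch-driven disintegration effect between entry and exit doors.
; Tick polls Switch.IsActive to run exit and entry door timelines in opposite directions and move and scale a grid Cube, reversing all three when inactive.
; The Cube's location and size feed a Material Parameter Collection.
; Door updates drive a DoOnce that applies a mask-test material to components tracked inside the trigger Box.
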(event OnComponentBeginOverlap(Box)
  (params (OverlappedComponent :type Primitive%20Component%20Object%20Reference) (OtherActor :type Actor%20Object%20Reference) (OtherComp :type Primitive%20Component%20Object%20Reference) (OtherBodyIndex :type Integer) (bFromSweep :type Boolean) (SweepResult :type Hit%20Result%20Structure%20%28by%20ref%29))
  (Utilities|Array|Add (Variables|Default|GetWithin%20Trigger) OtherComp))

(event OnComponentEndOverlap(Box)
  (params (OverlappedComponent :type Primitive%20Component%20Object%20Reference) (OtherActor :type Actor%20Object%20Reference) (OtherComp :type Primitive%20Component%20Object%20Reference) (OtherBodyIndex :type Integer))
  (Utilities|Array|RemoveItem (Variables|Default|GetWithin%20Trigger) OtherComp))

(event EventBeginPlay)

(event Collision|EventActorBeginOverlap
  (params (OtherActor :type Actor%20Object%20Reference)))

(event EventTick
  (params (DeltaSeconds :type Float%20%28single-precision%29))
  (bind _cube (Variables|Default|GetCube))
  (bind _returnvalue (Transformation|GetWorldScale _cube))
  (bind _returnvalue_2 (* _returnvalue 100))
  (bind (_x _y _z) (Math|Vector|BreakVector _returnvalue_2))
  (if (Variables|/Game/Blueprints/Parents/BP_CB_ParentDontUse_00.BP_CB_ParentDontUse_00_C|GetisActive (Variables|Default|GetSwitch))
    (Utilities|FlowControl|Sequence
      (:then_0
        (bind (_direction _leftdoor _rightdoor) (Timeline|Doors Play)
          (:Update
            (Transformation|SetRelativeLocation (Variables|Default|GetExitLeft) _leftdoor false false)
            (Transformation|SetRelativeLocation (Variables|Default|GetExitRight) _rightdoor false false)
            (goto _label Reset))))
      (:then_1
        (bind (_direction_2 _leftdoor_2 _rightdoor_2) (Timeline|Timeline_0 Reverse)
          (:Update
            (Transformation|SetRelativeLocation (Variables|Default|GetEntryLeft) _leftdoor_2 false false)
            (Transformation|SetRelativeLocation (Variables|Default|GetEntryright) _rightdoor_2 false false)
            (Utilities|FlowControl|DoOnce false :!label _label
              (:Completed
                (for _array_element (Variables|Default|GetWithin%20Trigger)
                  (Rendering|Material|SetMaterial _array_element 0 "/Game/Materials/Effects/M_CB_Spheremasktest.M_CB_SphereMaskTest")))))))
      (:then_2
        (bind (_direction_3 _gridmovement _gridscale) (Timeline|Timeline_1 Play)
          (:Update
            (Transformation|SetRelativeLocation (Variables|Default|GetCube) (Math|Vector|MakeVector 2.5e+02 -2.5e+02 _gridmovement) false false)
            (Transformation|SetRelativeScale3D _cube (Math|Vector|MakeVector 5.2 5.0 _gridscale))
            (Rendering|Material|SetVectorParameterValue "/Game/Materials/Effects/MPC_CB_DecontaminaionEffect.MPC_CB_DecontaminaionEffect" "Location" (Math|Conversions|ToLinearColor(Vector) (Transformation|GetWorldLocation _cube)) :!class /Script/Engine.KismetMaterialLibrary)
            (Rendering|Material|SetScalarParameterValue "/Game/Materials/Effects/MPC_CB_DecontaminaionEffect.MPC_CB_DecontaminaionEffect" "SizeX" _x :!class /Script/Engine.KismetMaterialLibrary)
            (Rendering|Material|SetScalarParameterValue "/Game/Materials/Effects/MPC_CB_DecontaminaionEffect.MPC_CB_DecontaminaionEffect" "SizeY" _y :!class /Script/Engine.KismetMaterialLibrary)
            (Rendering|Material|SetScalarParameterValue "/Game/Materials/Effects/MPC_CB_DecontaminaionEffect.MPC_CB_DecontaminaionEffect" "SizeZ" _z :!class /Script/Engine.KismetMaterialLibrary)))))
    (else
      (Utilities|FlowControl|Sequence
        (:then_0
          (Timeline|Doors Reverse))
        (:then_1
          (Timeline|Timeline_0 Play))
        (:then_2
          (Timeline|Timeline_1 Reverse))))))

(fn ConstructionScript
  (bind _cube (Variables|Default|GetCube))
  (Rendering|Material|SetVectorParameterValue "/Game/Materials/Effects/MPC_CB_DecontaminaionEffect.MPC_CB_DecontaminaionEffect" "Location" (Math|Conversions|ToLinearColor(Vector) (Transformation|GetWorldLocation _cube)) :!class /Script/Engine.KismetMaterialLibrary)
  (Rendering|Material|SetVectorParameterValue "/Game/Materials/Effects/MPC_CB_DecontaminaionEffect.MPC_CB_DecontaminaionEffect" "Size" (Math|Conversions|ToLinearColor(Vector) (Transformation|GetWorldScale _cube)) :!class /Script/Engine.KismetMaterialLibrary))