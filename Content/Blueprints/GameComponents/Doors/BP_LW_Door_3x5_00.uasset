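; Two-panel sliding door that opens when all of its linked laser receivers are active and closes otherwise.
; A looping timeline, with play rate set by PerformanceDelay, fires an event track to poll the receivers instead of using Tick.
; ReceiverChecker counts consecutive active receivers when RequiresPower is set.
; Its result plays or reverses DoorTimeLine, which drives both panels' relative locations.
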(event EventBeginPlay
  (Components|Timeline|SetPlayRate (Variables|Default|GetLooping) (Variables|Optimization|GetPerformanceDelay))
  (Timeline|Looping PlayFromStart
    (:NewTrack_1
      (bind _returnvalue (CallFunction|ReceiverChecker))
      (if _returnvalue
        (bind (_direction _door1 _door2) (Timeline|DoorTimeLine Play)
          (:Update
            (Utilities|FlowControl|Sequence
              (:then_0
                (Transformation|SetRelativeLocation (Variables|Default|GetDoor_L.1) _door2 false false))
              (:then_1
                (Transformation|SetRelativeLocation (Variables|Default|GetDoor_R.1) _door1 false false)))))
        (else
          (Variables|Default|SetActivated 0)
          (Timeline|DoorTimeLine Reverse))))))

(fn ConstructionScript)

(fn ReceiverChecker
  (bind _laserrecieverref (Variables|Configuration|GetLaserRecieverRef))
  (if (Variables|Configuration|GetRequiresPower)
    (Variables|Default|SetActivated 0)
    (for _array_element _laserrecieverref
      (if (Variables|/Game/Blueprints/Misc/Parents/BP_CB_ParentDontUse_00.BP_CB_ParentDontUse_00_C|GetisActive _array_element)
        (bind _result (Math|Integer|IncrementInt (Variables|Default|GetActivated))
          (:%20%20
            (Variables|Default|SetActivated _result)))
        (else
          (Variables|Default|SetActivated 0))))
    (return (>= (Variables|Default|GetActivated) (Utilities|Array|Length _laserrecieverref)))))