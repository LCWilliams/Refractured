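; Sliding double door that opens while all of its linked laser receivers are active and closes when any goes inactive.
; A looping timeline, rated by PerformanceDelay, polls ReceiverChecker and plays or reverses DoorTimeLine to move both panels.
; DoOnce gates on timeline direction trigger motor audio and a visible blocking cube, both cleared when movement finishes.
; ReceiverChecker's return-true node is unwired, so only doors with RequiresPower evaluate receivers.
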(event EventBeginPlay
  (bind _blockingcube (Variables|Default|GetBlockingCube))
  (bind _blockingcube_2 (Variables|Default|GetBlockingCube))
  (bind _blockingcube_3 (Variables|Default|GetBlockingCube))
  (bind _doormotorsaudio (Variables|Default|GetDoorMotorsAudio))
  (Utilities|FlowControl|Sequence
    (:then_0
      ;[1 1 0] Lazy fix for playing sound on play
      (bind _returnvalue (CallFunction|ReceiverChecker))
      (if (not _returnvalue)
        (Utilities|FlowControl|Delay 0.2)
        (Audio|Components|Audio|Stop (Variables|Default|GetDoorMotorsAudio))))
    (:then_1
      (Components|Timeline|SetPlayRate (Variables|Default|GetLooping) (Variables|Optimization|GetPerformanceDelay))
      (Timeline|Looping PlayFromStart
        (:NewTrack_1
          (bind _returnvalue_2 (CallFunction|ReceiverChecker))
          (if _returnvalue_2
            (Utilities|FlowControl|Sequence
              (:then_0
                (switch Utilities|FlowControl|Switch|SwitchonETimelineDirection (stale _direction) :!label _label
                  (:Forward
                    (Utilities|FlowControl|Sequence
                      (:then_0
                        (Utilities|FlowControl|DoOnce false :!label _label_2
                          (:Completed
                            _)))
                      (:then_1
                        (goto _label_3 Reset))))
                  (:Backward
                    (Utilities|FlowControl|Sequence
                      (:then_0
                        (Utilities|FlowControl|DoOnce true :!label _label_3
                          (:Completed
                            _)))
                      (:then_1
                        (goto _label_2 Reset)))))
                (Utilities|IsValid _doormotorsaudio
                  (:Is%20Valid
                    (Audio|Components|Audio|Play _doormotorsaudio 0.0)
                    (Rendering|SetVisibility _blockingcube_3 true false)
                    (Collision|SetCollisionEnabled _blockingcube_3 "QueryAndPhysics"))))
              (:then_1
                (bind (_direction _leftdoor _rightdoor) (Timeline|DoorTimeLine Play)
                  (:Update
                    (Transformation|SetRelativeLocation (Variables|Default|GetDoor_L.1) _leftdoor false false)
                    (Transformation|SetRelativeLocation (Variables|Default|GetDoor_R.1) _rightdoor false false))
                  (:Finished
                    (Audio|Components|Audio|Stop (Variables|Default|GetDoorMotorsAudio))
                    (Rendering|SetVisibility _blockingcube false false)
                    (Collision|SetCollisionEnabled _blockingcube "NoCollision")))))
            (else
              (Variables|Default|SetActivated 0)
              (Utilities|FlowControl|Sequence
                (:then_0
                  (goto _label))
                (:then_1
                  (Timeline|DoorTimeLine Reverse))))))))
    (:then_2
      (Rendering|SetVisibility _blockingcube_2 false false)
      (Collision|SetCollisionEnabled _blockingcube_2 "NoCollision"))))

(fn ConstructionScript)

(fn ReceiverChecker
  (bind _laserrecieverref (Variables|Configuration|GetLaserRecieverRef))
  (if (Variables|Configuration|GetRequiresPower)
    (Variables|Default|SetActivated 0)
    (for _array_element _laserrecieverref
      (if (Variables|/Game/Blueprints/Misc/Parents/BP_CB_ParentDontUse_00.BP_CB_ParentDontUse_00_C|GetisActive _array_element)
        (bind _result (Math|Integer|IncrementInt (Variables|Default|GetActivated))
          (:%20%20
            (Variables|Default|SetActivated _result)))
        (else
          (Variables|Default|SetActivated 0))))
    (return (>= (Variables|Default|GetActivated) (Utilities|Array|Length _laserrecieverref)))))