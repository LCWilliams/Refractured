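; Laser receiver switch that activates when hit by a laser of the required colour and power.
; Each tick it sets IsActive from the raycast component's active flag, a tolerance-based colour match and an exact power match.
; Activation drives a timeline that blends the receiver's dynamic material to its success look and plays a sound once; deactivation reverses both timeline and DoOnce state.
; The construction script shows the required colour and waiting state.
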(event EventTick
  (params (DeltaSeconds :type Float%20%28single-precision%29))
  (bind _bp_cb_raycast_component_00 (Variables|Default|GetBP_CB_Raycast_Component_00))
  (bind _audio (Variables|Default|GetAudio))
  ;[1 1 1] Sets Active if compared colour are close to equal
  (bind _output_get (Variables|Default|SetisActive (Math|Boolean|ANDBoolean (Variables|/Game/Blueprints/Misc/Components/BP_CB_Raycast_Component_00.BP_CB_Raycast_Component_00_C|GetSetObjectActive _bp_cb_raycast_component_00) (CallFunction|CompareColours (Variables|/Game/Blueprints/Misc/Components/BP_CB_Raycast_Component_00.BP_CB_Raycast_Component_00_C|GetSentColour _bp_cb_raycast_component_00) (Variables|Default|GetColourErrorTolerance) (Variables|Default|GetReqColour)) (== (Variables|/Game/Blueprints/Misc/Components/BP_CB_Raycast_Component_00.BP_CB_Raycast_Component_00_C|GetSentPower _bp_cb_raycast_component_00) (Variables|Default|GetRequiredPower)))))
  (if _output_get
    (Utilities|FlowControl|Sequence
      (:then_0
        (bind _timeline1 (Timeline|LerpTimeline Play)
          (:Update
            (CallFunction|LerpMaterialValues _timeline1))))
      (:then_1
        (Utilities|FlowControl|DoOnce true :!label _label
          (:Completed
            (Audio|Components|Audio|SetVolumeMultiplier _audio 3.0 :!class /Script/Engine.AudioComponent)
            (Audio|Components|Audio|Play _audio 0.0)))))
    (else
      (Utilities|FlowControl|Sequence
        (:then_0
          (Timeline|LerpTimeline Reverse))
        (:then_1
          (goto _label Reset))))))

(fn ConstructionScript
  (bind _receiver (Variables|Default|GetReceiver))
  ;[1 1 1] Sets Switch Colour
  (|CallParentFunction)
  (bind _returnvalue (Rendering|Material|CreateDynamicMaterialInstance _receiver 1 "/Game/Materials/Plains/ReceiverPlate/M_LW_ReceiverPlate_02.M_LW_ReceiverPlate_02" :!class /Script/Engine.PrimitiveComponent))
  (bind _output_get (Variables|Default|SetDynamicMaterial _returnvalue))
  (Rendering|Material|SetMaterial _receiver 1 _returnvalue)
  (Rendering|Material|SetVectorParameterValue _output_get "InputColour" (Variables|Default|GetReqColour) :!class /Script/Engine.MaterialInstanceDynamic)
  (if (== (Variables|Default|GetRequiredPower) 0)
    _
    (else
      (Rendering|Material|SetScalarParameterValue _output_get "LaserPower" 1.0 :!class /Script/Engine.MaterialInstanceDynamic)))
  (CallFunction|ApplyWaiting))

(fn ApplyWaiting
  (bind _dynamicmaterial (Variables|Default|GetDynamicMaterial))
  (Rendering|Material|SetVectorParameterValue _dynamicmaterial "InputColour" (Variables|Default|GetReqColour) :!class /Script/Engine.MaterialInstanceDynamic)
  (Rendering|Material|SetVectorParameterValue _dynamicmaterial "StatusColour" "(R=0.050000,G=0.050000,B=0.050000,A=1.000000)" :!class /Script/Engine.MaterialInstanceDynamic)
  (Rendering|Material|SetScalarParameterValue _dynamicmaterial "StatusSpinSpeed" 0.0 :!class /Script/Engine.MaterialInstanceDynamic)
  (Rendering|Material|SetScalarParameterValue _dynamicmaterial "ColourSpinSpeed" 0.0 :!class /Script/Engine.MaterialInstanceDynamic)
  (Rendering|Material|SetScalarParameterValue _dynamicmaterial "ColourPulseSpeed" 2.0 :!class /Script/Engine.MaterialInstanceDynamic))

(fn LerpMaterialValues
  (params (Lerp%20Value :type Float%20%28single-precision%29))
  (bind _dynamicmaterial (Variables|Default|GetDynamicMaterial))
  (Rendering|Material|SetVectorParameterValue _dynamicmaterial "StatusColour" (Math|Color|Lerp(LinearColor) "(R=0.010000,G=0.010000,B=0.010000,A=1.000000)" (Variables|Default|GetSuccessColour) Lerp%20Value) :!class /Script/Engine.MaterialInstanceDynamic)
  (Rendering|Material|SetScalarParameterValue _dynamicmaterial "StatusSpinSpeed" (Math|Float|Lerp 0.0 5.0 Lerp%20Value) :!class /Script/Engine.MaterialInstanceDynamic)
  (Rendering|Material|SetScalarParameterValue _dynamicmaterial "ColourSpinSpeed" (Math|Float|Lerp 0.0 1e+01 Lerp%20Value) :!class /Script/Engine.MaterialInstanceDynamic)
  (Rendering|Material|SetScalarParameterValue _dynamicmaterial "ColourPulseSpeed" (Math|Float|Lerp 3.0 0.0 Lerp%20Value) :!class /Script/Engine.MaterialInstanceDynamic))