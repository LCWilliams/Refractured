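; BP_CB_Switch_00 is a switch that follows its raycast component's active flag and plays a sound when toggled.
; Every Tick copies SetObjectActive from BPCBRaycastComponent00 into IsActive.
; Two DoOnce nodes, each reset by the opposite state, turn that polled value into edge triggers, so the shared Audio plays once per change rather than every frame.
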(event EventBeginPlay
  (|CallParentFunction))

(event EventTick
  (params (DeltaSeconds :type Float%20%28single-precision%29))
  ;[1 1 1] Toggles On Raycast
  (bind _output_get (Variables|Default|SetisActive (Variables|/Game/Blueprints/Misc/Components/BP_CB_Raycast_Component_00.BP_CB_Raycast_Component_00_C|GetSetObjectActive (Variables|Default|GetBP_CB_Raycast_Component_00))))
  (if _output_get
    (Utilities|FlowControl|Sequence
      (:then_0
        (Utilities|FlowControl|DoOnce false :!label _label
          (:Completed
            _)))
      (:then_1
        (goto _label_2 Reset)))
    (else
      (Utilities|FlowControl|Sequence
        (:then_0
          (Utilities|FlowControl|DoOnce true :!label _label_2
            (:Completed
              _)))
        (:then_1
          (goto _label Reset)))))
  (Audio|Components|Audio|Play (Variables|Default|GetAudio) 0.0))

(fn ConstructionScript
  (|CallParentFunction))