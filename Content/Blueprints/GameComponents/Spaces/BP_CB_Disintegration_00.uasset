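; Decontamination airlock that strips grabbable objects from the player passing between its entry and exit doors.
; The player entering the trigger closes the open doors, whose timeline then starts a disintegration sweep.
; The sweep moves a grid and box, feeding box bounds to a material parameter collection for the mask material applied to overlapping grabbables.
; When it finishes, tracked objects return to start, the player drops them and the opposite doors open.
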(event OnComponentBeginOverlap(Box1)
  (params (OverlappedComponent :type Primitive%20Component%20Object%20Reference) (OtherActor :type Actor%20Object%20Reference) (OtherComp :type Primitive%20Component%20Object%20Reference) (OtherBodyIndex :type Integer) (bFromSweep :type Boolean) (SweepResult :type Hit%20Result%20Structure%20%28by%20ref%29))
  ;[1 1 1] Starts Process When Player enters Trigger
  (if (== OtherActor (Game|Player|GetPlayerPawn 0))
    (switch Utilities|FlowControl|Switch|SwitchonE_CB_DisintegrationRoomState_00 (Variables|Default|GetRoomState)
      (:NewEnumerator0
        (CallFunction|CloseEntry))
      (:NewEnumerator2
        (CallFunction|CloseExit)))))

(event OnComponentBeginOverlap(Box)
  (params (OverlappedComponent :type Primitive%20Component%20Object%20Reference) (OtherActor :type Actor%20Object%20Reference) (OtherComp :type Primitive%20Component%20Object%20Reference) (OtherBodyIndex :type Integer) (bFromSweep :type Boolean) (SweepResult :type Hit%20Result%20Structure%20%28by%20ref%29))
  ;[1 1 1] Adds all objects with tag to an array and sets their material
  (if (CallFunction|Grabable OtherActor)
    (Utilities|Array|Add (Variables|Default|GetWithin%20Trigger) OtherActor)
    (Rendering|Material|SetMaterial OtherComp 0 "/Game/Materials/Effects/M_CB_Spheremasktest.M_CB_SphereMaskTest")))

(event OnComponentEndOverlap(Box)
  (params (OverlappedComponent :type Primitive%20Component%20Object%20Reference) (OtherActor :type Actor%20Object%20Reference) (OtherComp :type Primitive%20Component%20Object%20Reference) (OtherBodyIndex :type Integer))
  ;[1 1 1] Adds all objects with tag to an array and sets their material
  (if (CallFunction|Grabable OtherActor)
    (Utilities|Array|RemoveItem (Variables|Default|GetWithin%20Trigger) OtherActor)))

(event Custom|OpenEntry
  ;[1 1 1] Opens And Closes the entry doors when the events are called
  (bind (_direction _leftdoor _rightdoor) (Timeline|EntryDoorsTimeLine PlayFromStart)
    (:Update
      (Transformation|SetRelativeLocation (Variables|Default|GetEntryLeft) _leftdoor false false)
      (Transformation|SetRelativeLocation (Variables|Default|GetEntryright) _rightdoor false false))
    (:Finished
      (switch Utilities|FlowControl|Switch|SwitchonETimelineDirection _direction
        (:Backward
          (CallFunction|StartDisintegration))))))

(event Custom|CloseEntry
  ;[1 1 1] Opens And Closes the entry doors when the events are called
  (bind (_direction _leftdoor _rightdoor) (Timeline|EntryDoorsTimeLine ReverseFromEnd)
    (:Update
      (Transformation|SetRelativeLocation (Variables|Default|GetEntryLeft) _leftdoor false false)
      (Transformation|SetRelativeLocation (Variables|Default|GetEntryright) _rightdoor false false))
    (:Finished
      (switch Utilities|FlowControl|Switch|SwitchonETimelineDirection _direction
        (:Backward
          (CallFunction|StartDisintegration))))))

(event Custom|OpenExit
  ;[1 1 1] Opens And Closes the exit doors when the events are called
  (bind (_direction _leftdoor _rightdoor) (Timeline|ExitDoorsTimeline PlayFromStart)
    (:Update
      (Transformation|SetRelativeLocation (Variables|Default|GetExitLeft) _leftdoor false false)
      (Transformation|SetRelativeLocation (Variables|Default|GetExitRight) _rightdoor false false))
    (:Finished
      (switch Utilities|FlowControl|Switch|SwitchonETimelineDirection _direction
        (:Backward
          (CallFunction|StartDisintegration))))))

(event Custom|StartDisintegration
  (bind _box (Variables|Default|GetBox))
  (bind _returnvalue (Transformation|GetWorldScale _box))
  (bind _returnvalue_2 (* _returnvalue 100))
  (bind (_x _y _z) (Math|Vector|BreakVector _returnvalue_2))
  ;[1 1 1] Disentegration
  (bind (_direction _gridmovement _gridscale _vgridmovement) (Timeline|Disintegration%20Grid%20Timeline PlayFromStart)
    (:Update
      (Transformation|SetRelativeLocation (Variables|Default|GetCube) (Math|Vector|MakeVector 2.5e+02 -2.5e+02 _vgridmovement) false false)
      (Transformation|SetRelativeLocation (Variables|Default|GetBox) (Math|Vector|MakeVector 2.5e+02 -2.5e+02 _gridmovement) false false)
      (Transformation|SetRelativeScale3D _box (Math|Vector|MakeVector 5.2 5.0 _gridscale))
      (Rendering|Material|SetVectorParameterValue "/Game/Materials/Effects/MPC_CB_DecontaminaionEffect.MPC_CB_DecontaminaionEffect" "Location" (Math|Conversions|ToLinearColor(Vector) (Transformation|GetWorldLocation _box)) :!class /Script/Engine.KismetMaterialLibrary)
      (Rendering|Material|SetScalarParameterValue "/Game/Materials/Effects/MPC_CB_DecontaminaionEffect.MPC_CB_DecontaminaionEffect" "SizeX" _x :!class /Script/Engine.KismetMaterialLibrary)
      (Rendering|Material|SetScalarParameterValue "/Game/Materials/Effects/MPC_CB_DecontaminaionEffect.MPC_CB_DecontaminaionEffect" "SizeY" _y :!class /Script/Engine.KismetMaterialLibrary)
      (Rendering|Material|SetScalarParameterValue "/Game/Materials/Effects/MPC_CB_DecontaminaionEffect.MPC_CB_DecontaminaionEffect" "SizeZ" _z :!class /Script/Engine.KismetMaterialLibrary))
    (:Finished
      (for _array_element (Variables|Default|GetWithin%20Trigger)
        (Class|BPILWInterface|ResettoStartLocation(Message) _array_element)
        (Default|Drop (.AsBP%20CB%20Player%20Controller%2000 (Utilities|Casting|CastToBP_CB_PlayerController_00 (Game|Player|GetPlayerPawn 0)))))
      (switch Utilities|FlowControl|Switch|SwitchonE_CB_DisintegrationRoomState_00 (Variables|Default|GetRoomState)
        (:NewEnumerator0
          (Variables|Default|SetRoomState "NewEnumerator2")
          (CallFunction|OpenExit))
        (:NewEnumerator2
          (Variables|Default|SetRoomState "NewEnumerator0")
          (CallFunction|OpenEntry)))
      (CallFunction|ResetDisentegration))))

(event Custom|ResetDisentegration
  (bind _box (Variables|Default|GetBox))
  (bind _returnvalue (Transformation|GetWorldScale _box))
  (bind _returnvalue_2 (* _returnvalue 100))
  (bind (_x _y _z) (Math|Vector|BreakVector _returnvalue_2))
  ;[1 1 1] Disentegration
  (bind (_direction _gridmovement _gridscale _vgridmovement) (Timeline|Disintegration%20Grid%20Timeline SetNewTime)
    (:Update
      (Transformation|SetRelativeLocation (Variables|Default|GetCube) (Math|Vector|MakeVector 2.5e+02 -2.5e+02 _vgridmovement) false false)
      (Transformation|SetRelativeLocation (Variables|Default|GetBox) (Math|Vector|MakeVector 2.5e+02 -2.5e+02 _gridmovement) false false)
      (Transformation|SetRelativeScale3D _box (Math|Vector|MakeVector 5.2 5.0 _gridscale))
      (Rendering|Material|SetVectorParameterValue "/Game/Materials/Effects/MPC_CB_DecontaminaionEffect.MPC_CB_DecontaminaionEffect" "Location" (Math|Conversions|ToLinearColor(Vector) (Transformation|GetWorldLocation _box)) :!class /Script/Engine.KismetMaterialLibrary)
      (Rendering|Material|SetScalarParameterValue "/Game/Materials/Effects/MPC_CB_DecontaminaionEffect.MPC_CB_DecontaminaionEffect" "SizeX" _x :!class /Script/Engine.KismetMaterialLibrary)
      (Rendering|Material|SetScalarParameterValue "/Game/Materials/Effects/MPC_CB_DecontaminaionEffect.MPC_CB_DecontaminaionEffect" "SizeY" _y :!class /Script/Engine.KismetMaterialLibrary)
      (Rendering|Material|SetScalarParameterValue "/Game/Materials/Effects/MPC_CB_DecontaminaionEffect.MPC_CB_DecontaminaionEffect" "SizeZ" _z :!class /Script/Engine.KismetMaterialLibrary))
    (:Finished
      (for _array_element (Variables|Default|GetWithin%20Trigger)
        (Class|BPILWInterface|ResettoStartLocation(Message) _array_element)
        (Default|Drop (.AsBP%20CB%20Player%20Controller%2000 (Utilities|Casting|CastToBP_CB_PlayerController_00 (Game|Player|GetPlayerPawn 0)))))
      (switch Utilities|FlowControl|Switch|SwitchonE_CB_DisintegrationRoomState_00 (Variables|Default|GetRoomState)
        (:NewEnumerator0
          (Variables|Default|SetRoomState "NewEnumerator2")
          (CallFunction|OpenExit))
        (:NewEnumerator2
          (Variables|Default|SetRoomState "NewEnumerator0")
          (CallFunction|OpenEntry)))
      (CallFunction|ResetDisentegration))))

(event Custom|CloseExit
  ;[1 1 1] Opens And Closes the exit doors when the events are called
  (bind (_direction _leftdoor _rightdoor) (Timeline|ExitDoorsTimeline ReverseFromEnd)
    (:Update
      (Transformation|SetRelativeLocation (Variables|Default|GetExitLeft) _leftdoor false false)
      (Transformation|SetRelativeLocation (Variables|Default|GetExitRight) _rightdoor false false))
    (:Finished
      (switch Utilities|FlowControl|Switch|SwitchonETimelineDirection _direction
        (:Backward
          (CallFunction|StartDisintegration))))))

(event EventBeginPlay
  ;[1 1 1] Open Starting Door
  (switch Utilities|FlowControl|Switch|SwitchonE_CB_DisintegrationRoomState_00 (Variables|Default|GetRoomState)
    (:NewEnumerator0
      (CallFunction|OpenEntry))
    (:NewEnumerator2
      (CallFunction|OpenExit))))

(fn ConstructionScript
  (bind _cube (Variables|Default|GetCube))
  (Rendering|Material|SetVectorParameterValue "/Game/Materials/Effects/MPC_CB_DecontaminaionEffect.MPC_CB_DecontaminaionEffect" "Location" (Math|Conversions|ToLinearColor(Vector) (Transformation|GetWorldLocation _cube)) :!class /Script/Engine.KismetMaterialLibrary)
  (Rendering|Material|SetVectorParameterValue "/Game/Materials/Effects/MPC_CB_DecontaminaionEffect.MPC_CB_DecontaminaionEffect" "Size" (Math|Conversions|ToLinearColor(Vector) (Transformation|GetWorldScale _cube)) :!class /Script/Engine.KismetMaterialLibrary))