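; Laser hub that fires a coloured, bouncing beam and can be possessed by the player to aim it.
; A rate-adjustable looping timeline replaces Tick for firing, optionally gated by receivers (inverted by StartsActive), using beam particles pre-spawned per bounce.
; Power state fades linked splines and drives looping sound; shutdown clears the last hit target.
; Aim input rotates skeletal bones with yaw wrap and pitch clamp, updating the laser UI.
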(event Custom|RemotePossess
  (bind _asbp_cb_player_controller_00 (Utilities|Casting|CastToBP_CB_PlayerController_00 (Game|Player|GetPlayerPawn 0)))
  (bind _output_get (Variables|Default|SetPlayer%20Controller _asbp_cb_player_controller_00))
  (Default|TogglePossesion _output_get true self))

(event EventTick
  (params (DeltaSeconds :type Float%20%28single-precision%29))
  ;[1 1 1] Laser Pawn Possession
  (if (Variables|Config|GetControllable)
    (bind _raycastcomponent (PlayerControl|Possession))))

(event EventBeginPlay
  (bind _laserparticlearray (Variables|Laser|GetLaserParticleArray))
  (bind _sc_laserhub (Variables|Default|GetSC_Laserhub))
  (bind _bp_cb_laser_component_01 (Variables|Default|GetBP_CB_Laser_Component_01))
  (bind _bp_cb_laser_component_01_2 (Variables|Default|GetBP_CB_Laser_Component_01))
  (bind _sc_laserhub_2 (Variables|Default|GetSC_Laserhub))
  ;[1 1 1] Initialise Components
  (Utilities|FlowControl|Sequence
    (:then_0
      (Utilities|Construction))
    (:then_1
      (Default|TraceSetup _bp_cb_laser_component_01 _bp_cb_laser_component_01)
      (if (== (Variables|Config|GetLaserPower) 0)
        (Variables|/Script/Engine.AudioComponent|SetLowPassFilterFrequency _sc_laserhub_2 1e+04)
        (else
          (Variables|/Script/Engine.AudioComponent|SetLowPassFilterFrequency _sc_laserhub_2 1.9e+04))))
    (:then_2
      ;[1 1 1] Event Tick Replacer
      (Components|Timeline|SetPlayRate (Variables|Default|GetLooping) (Variables|Default|GetPerformanceDelay))
      (Timeline|Looping PlayFromStart
        (:Tick
          ;[1 1 1] Raycast
          (if (not (Variables|Default|GetPENDING%20DELETION))
            (Adjustments|CameraLaserRotation)
            (if (Variables|Config|GetNeedsPower)
              (bind _returnvalue (CallFunction|CheckReceivers (Variables|Config|GetReceiverRef)))
              (if (select (Variables|Config|GetStartsActive) (not _returnvalue) _returnvalue)
                (bind _hitreceiver (Default|FireLaser _bp_cb_laser_component_01 _bp_cb_laser_component_01 (Variables|Config|GetLaserColour) _laserparticlearray (Variables|Config|GetMaxBounce) (Variables|Config|GetLaserPower) :!label _label))
                (Variables|Activation|SetLaserIsActive true)
                (Utilities|FlowControl|Sequence
                  (:then_0
                    (bind _newtrack_0 (Timeline|Timeline_0 Play)
                      (:Update
                        (for _array_element (Variables|Config|GetSplineActors)
                          (Variables|/Game/Blueprints/SplineActor.SplineActor_C|SetStrength _array_element (Math|Float|Lerp 0.2 1.0 _newtrack_0))))))
                  (:then_1
                    (Utilities|CancelLoop 19.5 :!label _label_2
                      (:Execute
                        (Audio|Components|Audio|Play _sc_laserhub 0.0)
                        (goto _label_3 Reset)))))
                (else
                  (Utilities|FlowControl|Sequence
                    (:then_0
                      (Utilities|FlowControl|DoOnce false :!label _label_3
                        (:Completed
                          (Default|DisableLasers _bp_cb_laser_component_01_2 _laserparticlearray)
                          (Utilities|FlowControl|Sequence
                            (:then_0
                              (goto _label_2 Stop))
                            (:then_1
                              (Audio|Components|Audio|Stop _sc_laserhub)
                              (Utilities|IsValid _hitreceiver
                                (:Is%20Valid
                                  (Default|InputActive (Variables|/Game/Blueprints/Misc/Parents/BP_CB_ParentDontUse_00.BP_CB_ParentDontUse_00_C|GetBP_CB_Raycast_Component_00 _hitreceiver) false)
                                  (Default|ResetLaserHitRef _bp_cb_laser_component_01_2))))))))
                    (:then_1
                      (Variables|Activation|SetLaserIsActive false)
                      (Timeline|Timeline_0 Reverse)))))
              (else
                (goto _label)))))))))

(event Input|ActionEvents|InputActionActivate
  (params (Key :type Key%20Structure :default "AnyKey"))
  ;[1 1 1] Laser Pawn Possession
  (:Pressed
    (Variables|/Game/Blueprints/Misc/Components/BP_CB_Raycast_Component_00.BP_CB_Raycast_Component_00_C|SetSetObjectActive (stale EventTick _raycastcomponent) false)
    (CallFunction|DisableLaserUI)
    (Pawn|Possess (Game|GetPlayerController 0) (Variables|Default|GetPlayer%20Controller))))

(event Input|AxisEvents|InputAxisTurn
  (params (AxisValue :type Float%20%28single-precision%29))
  ;[1 1 1] Laser Rotation [Mouse]
  (bind _output_get (PlayerControl|RotationYaw AxisValue (Variables|/Game/Blueprints/GameComponents/Player/BP_CB_PlayerController_00.BP_CB_PlayerController_00_C|GetLaser%20Rotation%20Speed:%20Z (Variables|Default|GetPlayer%20Controller)) (Utilities|Time|GetWorldDeltaSeconds) (Variables|Default|GetSkM_LW_Laser_01_LaserBase))))

(event Input|AxisEvents|InputAxisLookUp
  (params (AxisValue :type Float%20%28single-precision%29))
  ;[1 1 1] Laser Rotation [Mouse]
  (PlayerControl|RotationPitch (stale Input|AxisEvents|InputAxisTurn _output_get) AxisValue (Variables|/Game/Blueprints/GameComponents/Player/BP_CB_PlayerController_00.BP_CB_PlayerController_00_C|GetLaser%20Rotation%20Speed:%20X (Variables|Default|GetPlayer%20Controller)) (Utilities|Time|GetWorldDeltaSeconds) (Variables|Default|GetSkM_LW_Laser_01_LaserBase)))

(event Input|AxisEvents|InputAxisTurnRate
  (params (AxisValue :type Float%20%28single-precision%29))
  ;[1 1 1] Laser Rotation [Mouse]
  (bind _output_get (PlayerControl|RotationYaw AxisValue (Variables|/Game/Blueprints/GameComponents/Player/BP_CB_PlayerController_00.BP_CB_PlayerController_00_C|GetLaser%20Rotation%20Speed:%20Z (Variables|Default|GetPlayer%20Controller)) (Utilities|Time|GetWorldDeltaSeconds) (Variables|Default|GetSkM_LW_Laser_01_LaserBase))))

(event Input|AxisEvents|InputAxisLookUpRate
  (params (AxisValue :type Float%20%28single-precision%29))
  ;[1 1 1] Laser Rotation [Mouse]
  (PlayerControl|RotationPitch (stale Input|AxisEvents|InputAxisTurnRate _output_get) AxisValue (Variables|/Game/Blueprints/GameComponents/Player/BP_CB_PlayerController_00.BP_CB_PlayerController_00_C|GetLaser%20Rotation%20Speed:%20X (Variables|Default|GetPlayer%20Controller)) (Utilities|Time|GetWorldDeltaSeconds) (Variables|Default|GetSkM_LW_Laser_01_LaserBase)))

(fn ConstructionScript
  (bind _skm_lw_laser_01_laserbase (Variables|Default|GetSkM_LW_Laser_01_LaserBase))
  (Transformation|AttachComponentToComponent (Variables|Default|GetCable) _skm_lw_laser_01_laserbase "Socket_LaserBody" "SnapToTarget" "SnapToTarget" "SnapToTarget" true)
  (Transformation|AttachComponentToComponent (Variables|Default|GetBP_CB_Laser_Component_01) _skm_lw_laser_01_laserbase "Socket_LaserOrigin" "SnapToTarget" "SnapToTarget" "SnapToTarget" false)
  (Transformation|AttachComponentToComponent (Variables|Default|GetCamera) _skm_lw_laser_01_laserbase "Socket_LaserCamera" "SnapToTarget" "SnapToTarget" "SnapToTarget" false)
  (for _array_element (Variables|Config|GetSplineActors)
    (Variables|/Game/Blueprints/SplineActor.SplineActor_C|SetSplineColour _array_element (Variables|Config|GetLaserColour))))

(fn Possession
  (bind _bp_cb_raycast_component_00 (Variables|Default|GetBP_CB_Raycast_Component_00))
  (bind _setobjectactive (Variables|/Game/Blueprints/Misc/Components/BP_CB_Raycast_Component_00.BP_CB_Raycast_Component_00_C|GetSetObjectActive _bp_cb_raycast_component_00))
  (if (Variables|Config|GetRemotePossesion)
    _
    (elif _setobjectactive
      (bind _asbp_cb_player_controller_00 (Utilities|Casting|CastToBP_CB_PlayerController_00 (Game|Player|GetPlayerPawn 0))
        (:then
          (bind _output_get (Variables|Default|SetPlayer%20Controller _asbp_cb_player_controller_00))
          (Default|TogglePossesion _output_get _setobjectactive self))
        (:CastFailed
          _))))
  (return _bp_cb_raycast_component_00))

(fn RotationYaw
  (params (InputAxis :type Float%20%28single-precision%29) (RotationSpeedModifier :type Float%20%28single-precision%29) (DeltaSeconds :type Float%20%28single-precision%29) (SkelatalMesh :type Poseable%20Mesh%20Component%20Object%20Reference))
  (bind _output_get (Variables|Rotation|SetCurrent%20Yaw (CallFunction|LimitYaw (+ (Variables|Rotation|GetCurrent%20Yaw) (* InputAxis RotationSpeedModifier DeltaSeconds)) InputAxis)))
  (Components|PoseableMesh|SetBoneRotationbyName SkelatalMesh "LaserBody" (Math|Rotator|MakeRotator 9e+01 0.0 _output_get) "ComponentSpace")
  (Default|SetBottomBarPosition (Variables|/Game/Blueprints/GameComponents/Player/BP_CB_PlayerController_00.BP_CB_PlayerController_00_C|GetLaserUIReference (Variables|Default|GetPlayer%20Controller)) (Math|Float|NormalizetoRange _output_get 0.0 359.0) _output_get)
  (return _output_get))

(fn RotationPitch
  (params (RotationYaw :type Float%20%28single-precision%29) (InputAxis :type Float%20%28single-precision%29) (RotationSpeedModifier :type Float%20%28single-precision%29) (DeltaSeconds :type Float%20%28single-precision%29) (SkelatalMesh :type Poseable%20Mesh%20Component%20Object%20Reference))
  (bind _output_get (Variables|Rotation|SetCurrent%20Pitch (+ (stale _output_get) (* InputAxis RotationSpeedModifier DeltaSeconds -1.0))))
  (bind _output_get_2 (Variables|Rotation|SetCurrent%20Pitch (Math|Float|Clamp(Float) _output_get 1.5e+02 2.4e+02)))
  (Components|PoseableMesh|SetBoneRotationbyName SkelatalMesh "LaserHead" (Math|Rotator|MakeRotator _output_get_2 1.8e+02 RotationYaw) "ComponentSpace")
  (Default|SetSidebarPosition (Variables|/Game/Blueprints/GameComponents/Player/BP_CB_PlayerController_00.BP_CB_PlayerController_00_C|GetLaserUIReference (Variables|Default|GetPlayer%20Controller)) (Math|Float|NormalizetoRange _output_get_2 1.5e+02 2.4e+02) _output_get_2))

(fn DivideRotator
  (params (InputRotation :type Rotator))
  (bind (_roll _pitch _yaw) (Math|Rotator|BreakRotator InputRotation))
  (bind _rotationcorector (LocalVariables|GetRotationCorector))
  (return (Math|Rotator|MakeRotator (/ _roll _rotationcorector) (/ _pitch _rotationcorector) (/ _yaw _rotationcorector))))

(fn CameraLaserRotation
  (bind _skm_lw_laser_01_laserbase (Variables|Default|GetSkM_LW_Laser_01_LaserBase))
  (Transformation|SetRelativeRotation (Variables|Default|GetBP_CB_Laser_Component_01) (Adjustments|DivideRotator (Transformation|GetSocketRotation _skm_lw_laser_01_laserbase "Socket_LaserOrigin")) false false)
  (Transformation|SetRelativeRotation (Variables|Default|GetCamera) (Adjustments|DivideRotator (Transformation|GetSocketRotation _skm_lw_laser_01_laserbase "Socket_LaserCamera")) false false))

(fn DisableLaserUI
  (bind _player_controller (Variables|Default|GetPlayer%20Controller))
  (bind _laseruireference (Variables|/Game/Blueprints/GameComponents/Player/BP_CB_PlayerController_00.BP_CB_PlayerController_00_C|GetLaserUIReference _player_controller))
  (Default|ToggleCrosshair (Variables|/Game/Blueprints/GameComponents/Player/BP_CB_PlayerController_00.BP_CB_PlayerController_00_C|GetPersistentUI _player_controller) true)
  (Widget|SetIsEnabled (Variables|/Game/Blueprints/GameComponents/Player/BP_CB_PlayerController_00.BP_CB_PlayerController_00_C|GetGameUIReference _player_controller) true)
  (UserInterface|Animation|PlayAnimation _laseruireference (Variables|/Game/Blueprints/GameComponents/Player/GraphicalUserInterface/BP_LW_LaserHub.BP_LW_LaserHub_C|GetInitialising _laseruireference) 0.0 1 "Reverse" 1.0))

(fn LimitYaw
  (params (Yaw :type Float%20%28single-precision%29%20%28by%20ref%29) (Input%20Direction :type Float%20%28single-precision%29%20%28by%20ref%29))
  (if (> Input%20Direction 0.1) ; True = + | False = -
    (if (>= Yaw 3.6e+02)
      (return 1.0)
      (else
        (return Yaw)))
    (elif (< Input%20Direction -0.1)
      (if (<= Yaw 0.0)
        (return 359.0)
        (else
          (return Yaw)))
      (else
        (return Yaw)))))