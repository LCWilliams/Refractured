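; Laser puzzle cube with six configurable faces (reflect, input, refract, dispersion) that the player can possess and rotate when Controllable.
; Construction sets face meshes and dynamic materials, and BeginPlay spawns pooled laser particles.
; While the raycast component has input, Tick fires refract faces in the held colour and dispersion faces in their own colour if the held colour covers it per channel.
; A timeline fades face materials with power, and lasers reset on input loss.
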(event EventTick
  (params (DeltaSeconds :type Float%20%28single-precision%29))
  (bind _bp_cb_raycast_component_00 (Variables|Default|GetBP_CB_Raycast_Component_00))
  (bind _inputamount (Variables|/Game/Blueprints/Misc/Components/BP_CB_Raycast_Component_00.BP_CB_Raycast_Component_00_C|GetInputAmount _bp_cb_raycast_component_00))
  (bind _returnvalue (> _inputamount 0))
  ;[1 1 1] Cube Behaviour
  (Utilities|FlowControl|Sequence
    (:then_0
      (if _returnvalue
        (Utilities|FlowControl|Sequence
          (:then_0
            (Variables|PassThroughVariables|SetInputPower (Variables|/Game/Blueprints/Misc/Components/BP_CB_Raycast_Component_00.BP_CB_Raycast_Component_00_C|GetSentPower _bp_cb_raycast_component_00))
            (Utilities|UpdateFaces)
            (Variables|Default|SetisActive true))
          (:then_1
            (goto _label Reset)))
        (else
          (Utilities|FlowControl|DoOnce false :!label _label
            (:Completed
              (Utilities|DisableLasers
                (:Out
                  (Variables|Default|SetisActive true))))))))
    (:then_1
      (if _returnvalue
        ;[1 1 1] Update Visuals on Faces
        (bind _timeline1 (Timeline|Timeline_1 Play)
          (:Update
            (Utilities|LerpMaterialValues _timeline1)))
        (else
          (Timeline|Timeline_1 Reverse))))
    (:then_2
      ;[1 1 1] Possession
      (if (Variables|Settings|GetControllable)
        (bind _raycastcomp (CallFunction|Possesion))))))

(event EventBeginPlay
  ;[1 1 1] Make Visual Lasers
  (for (_ _array_index) (Variables|Settings|GetFaceSettings)
    (bind _laserparticlearray (CallFunction|InstantiateLasers (Variables|PassThroughVariables|GetMaxBounce) (Variables|Settings|GetLaser%20Particle%20Template) false (Transformation|GetActorLocation self)))
    (Setup|AddLaserstoFace _array_index _laserparticlearray)))

(event Input|ActionEvents|InputActionActivate
  (params (Key :type Key%20Structure :default "AnyKey"))
  ;[1 1 1] Possession
  (:Pressed
    (Variables|/Game/Blueprints/Misc/Components/BP_CB_Raycast_Component_00.BP_CB_Raycast_Component_00_C|SetSetObjectActive (stale EventTick _raycastcomp) false)
    (Pawn|Possess (Game|GetPlayerController 0) (Variables|Default|GetPlayer%20Controller))))

(event Input|AxisEvents|InputAxisTurn
  (params (AxisValue :type Float%20%28single-precision%29))
  (bind _returnvalue (Utilities|Time|GetWorldDeltaSeconds))
  (bind _player_controller (Variables|Default|GetPlayer%20Controller))
  (Transformation|AddRelativeRotation (Variables|Default|GetSM_MC_UnicornCube_Frame_001) (Math|Rotator|MakeRotator 0.0 (* (stale Input|AxisEvents|InputAxisLookUp AxisValue) (Variables|/Game/Blueprints/GameComponents/Player/BP_CB_PlayerController_00.BP_CB_PlayerController_00_C|GetLaser%20Rotation%20Speed:%20Z _player_controller) _returnvalue -1.0) (* AxisValue _returnvalue (Variables|/Game/Blueprints/GameComponents/Player/BP_CB_PlayerController_00.BP_CB_PlayerController_00_C|GetLaser%20Rotation%20Speed:%20X _player_controller))) false false))

(event Input|AxisEvents|InputAxisLookUp
  (params (AxisValue :type Float%20%28single-precision%29))
  (bind _returnvalue (Utilities|Time|GetWorldDeltaSeconds))
  (bind _player_controller (Variables|Default|GetPlayer%20Controller))
  (Transformation|AddRelativeRotation (Variables|Default|GetSM_MC_UnicornCube_Frame_001) (Math|Rotator|MakeRotator 0.0 (* AxisValue (Variables|/Game/Blueprints/GameComponents/Player/BP_CB_PlayerController_00.BP_CB_PlayerController_00_C|GetLaser%20Rotation%20Speed:%20Z _player_controller) _returnvalue -1.0) (* (stale Input|AxisEvents|InputAxisTurn AxisValue) _returnvalue (Variables|/Game/Blueprints/GameComponents/Player/BP_CB_PlayerController_00.BP_CB_PlayerController_00_C|GetLaser%20Rotation%20Speed:%20X _player_controller))) false false))

(event Input|AxisEvents|InputAxisTurnRate
  (params (AxisValue :type Float%20%28single-precision%29))
  (bind _returnvalue (Utilities|Time|GetWorldDeltaSeconds))
  (bind _player_controller (Variables|Default|GetPlayer%20Controller))
  (Transformation|AddRelativeRotation (Variables|Default|GetSM_MC_UnicornCube_Frame_001) (Math|Rotator|MakeRotator 0.0 (* AxisValue (Variables|/Game/Blueprints/GameComponents/Player/BP_CB_PlayerController_00.BP_CB_PlayerController_00_C|GetLaser%20Rotation%20Speed:%20Z _player_controller) _returnvalue -1.0) (* (stale Input|AxisEvents|InputAxisLookUpRate AxisValue) _returnvalue (Variables|/Game/Blueprints/GameComponents/Player/BP_CB_PlayerController_00.BP_CB_PlayerController_00_C|GetLaser%20Rotation%20Speed:%20X _player_controller))) false false))

(event Input|AxisEvents|InputAxisLookUpRate
  (params (AxisValue :type Float%20%28single-precision%29))
  (bind _returnvalue (Utilities|Time|GetWorldDeltaSeconds))
  (bind _player_controller (Variables|Default|GetPlayer%20Controller))
  (Transformation|AddRelativeRotation (Variables|Default|GetSM_MC_UnicornCube_Frame_001) (Math|Rotator|MakeRotator 0.0 (* (stale Input|AxisEvents|InputAxisTurnRate AxisValue) (Variables|/Game/Blueprints/GameComponents/Player/BP_CB_PlayerController_00.BP_CB_PlayerController_00_C|GetLaser%20Rotation%20Speed:%20Z _player_controller) _returnvalue -1.0) (* AxisValue _returnvalue (Variables|/Game/Blueprints/GameComponents/Player/BP_CB_PlayerController_00.BP_CB_PlayerController_00_C|GetLaser%20Rotation%20Speed:%20X _player_controller))) false false))

(fn ConstructionScript
  (bind _dynamicmaterial (Variables|Default|GetDynamicMaterial))
  (Setup|CreateFaces)
  (for (_array_element _array_index) (Variables|Settings|GetFaces)
    (bind _returnvalue (Rendering|Material|CreateDynamicMaterialInstance _array_element 1 "/Game/Materials/Plains/ReceiverPlate/M_LW_ReceiverPlate_02.M_LW_ReceiverPlate_02" :!class /Script/Engine.PrimitiveComponent))
    (Utilities|Array|SetArrayElem _dynamicmaterial _array_index _returnvalue)
    (switch Utilities|FlowControl|Switch|SwitchonE_LW_Cube_01 (Utilities|Array|Get(acopy) (Variables|Settings|GetFaceSettings) _array_index)
      (:NewEnumerator1
        (Rendering|Material|SetMaterial _array_element 1 (Utilities|Array|Get(acopy) _dynamicmaterial _array_index) :!label _label)
        (Rendering|Material|SetVectorParameterValue :self (Utilities|Array|Get(acopy) _dynamicmaterial _array_index) :ParameterName "InputColour" :!class /Script/Engine.MaterialInstanceDynamic)
        (Rendering|Material|SetVectorParameterValue (Utilities|Array|Get(acopy) _dynamicmaterial _array_index) "StatusColour" "(R=0.050000,G=0.050000,B=0.050000,A=1.000000)" :!class /Script/Engine.MaterialInstanceDynamic)
        (Rendering|Material|SetScalarParameterValue (Utilities|Array|Get(acopy) _dynamicmaterial _array_index) "StatusSpinSpeed" 0.0 :!class /Script/Engine.MaterialInstanceDynamic)
        (Rendering|Material|SetScalarParameterValue (Utilities|Array|Get(acopy) _dynamicmaterial _array_index) "ColourSpinSpeed" 0.0 :!class /Script/Engine.MaterialInstanceDynamic)
        (Rendering|Material|SetScalarParameterValue (Utilities|Array|Get(acopy) _dynamicmaterial _array_index) "ColourPulseSpeed" 2.0 :!class /Script/Engine.MaterialInstanceDynamic))
      (:NewEnumerator2
        (goto _label))
      (:NewEnumerator3
        (Rendering|Material|SetMaterial _array_element 1 (Utilities|Array|Get(acopy) _dynamicmaterial _array_index))
        (Rendering|Material|SetVectorParameterValue (Utilities|Array|Get(acopy) _dynamicmaterial _array_index) "InputColour" (Utilities|Select :Index _array_index :Option%200 (Variables|DispersionValues|GetFrontDispersion) :Option%201 (Variables|DispersionValues|GetBackDispersion) :Option%202 (Variables|DispersionValues|GetLeftDispersion) :Option%203 (Variables|DispersionValues|GetRightDispersion) :Option%204 (Variables|DispersionValues|GetTopDispersion) :Option%205 (Variables|DispersionValues|GetBottomDispersion)) :!class /Script/Engine.MaterialInstanceDynamic)
        (Rendering|Material|SetVectorParameterValue (Utilities|Array|Get(acopy) _dynamicmaterial _array_index) "StatusColour" "(R=0.050000,G=0.050000,B=0.050000,A=1.000000)" :!class /Script/Engine.MaterialInstanceDynamic)
        (Rendering|Material|SetScalarParameterValue (Utilities|Array|Get(acopy) _dynamicmaterial _array_index) "StatusSpinSpeed" 0.0 :!class /Script/Engine.MaterialInstanceDynamic)
        (Rendering|Material|SetScalarParameterValue (Utilities|Array|Get(acopy) _dynamicmaterial _array_index) "ColourSpinSpeed" 0.0 :!class /Script/Engine.MaterialInstanceDynamic)
        (Rendering|Material|SetScalarParameterValue (Utilities|Array|Get(acopy) _dynamicmaterial _array_index) "ColourPulseSpeed" 2.0 :!class /Script/Engine.MaterialInstanceDynamic)))))

(fn CreateFaces
  (Variables|Settings|SetLaserComponents (Utilities|Array|MakeArray (Variables|Component:LaserComponent|GetLaserComponent_Front) (Variables|Component:LaserComponent|GetLaserComponent_Back) (Variables|Component:LaserComponent|GetLaserComponent_Left) (Variables|Component:LaserComponent|GetLaserComponent_Right) (Variables|Component:LaserComponent|GetLaserComponent_Top) (Variables|Component:LaserComponent|GetLaserComponent_Bottom)))
  (Variables|Settings|SetFaces (Utilities|Array|MakeArray (Variables|Default|GetFace_Front) (Variables|Default|GetFace_Back) (Variables|Default|GetFace_Left) (Variables|Default|GetFace_Right) (Variables|Default|GetFace_Top) (Variables|Default|GetFace_Bottom)))
  (bind _output_get (Variables|Settings|SetFaceSettings (Utilities|Array|MakeArray (Variables|Settings|GetFront) (Variables|Settings|GetBack) (Variables|Settings|GetLeft) (Variables|Settings|GetRight) (Variables|Settings|GetTop) (Variables|Settings|GetBottom))))
  (for (_array_element _array_index) _output_get
    (switch Utilities|FlowControl|Switch|SwitchonE_LW_Cube_01 _array_element
      (:NewEnumerator4
        (Components|StaticMesh|SetStaticMesh (Utilities|Array|Get(acopy) (Variables|Settings|GetFaces) _array_index) (Variables|Settings|GetReflectionFace)))
      (:NewEnumerator1
        (Components|StaticMesh|SetStaticMesh (Utilities|Array|Get(acopy) (Variables|Settings|GetFaces) _array_index) (Variables|Settings|GetInputFace)))
      (:NewEnumerator2
        (Components|StaticMesh|SetStaticMesh (Utilities|Array|Get(acopy) (Variables|Settings|GetFaces) _array_index) (Variables|Settings|GetOutputFace)))
      (:NewEnumerator3
        (Components|StaticMesh|SetStaticMesh (Utilities|Array|Get(acopy) (Variables|Settings|GetFaces) _array_index) (Variables|Settings|GetOutputFace))))))

(fn AddLaserstoFace
  (params (Loop%20Index :type Integer) (Particles%20To%20Add :type Array%20of%20Particle%20System%20Component%20Object%20References))
  (for _array_element 0
    (Utilities|Array|Add (Variables|FaceParticles|GetAllLasers) _array_element)))

(fn MakeDispersionSettings
  (params (FaceIndex :type Integer))
  (Utilities|FlowControl|Sequence
    (:then_0
      (switch int FaceIndex
        (:0
          (switch Utilities|FlowControl|Switch|SwitchonE_LW_Cube_01 (Variables|Settings|GetFront)))
        (:1
          (switch Utilities|FlowControl|Switch|SwitchonE_LW_Cube_01 (Variables|Settings|GetBack)))
        (:2
          (switch Utilities|FlowControl|Switch|SwitchonE_LW_Cube_01 (Variables|Settings|GetLeft)))
        (:3
          (switch Utilities|FlowControl|Switch|SwitchonE_LW_Cube_01 (Variables|Settings|GetRight)))
        (:4
          (switch Utilities|FlowControl|Switch|SwitchonE_LW_Cube_01 (Variables|Settings|GetTop)))
        (:5
          (switch Utilities|FlowControl|Switch|SwitchonE_LW_Cube_01 (Variables|Settings|GetBottom)))))))

(fn RefractS
  (params (Array%20Index :type Integer%20%28by%20ref%29))
  (bind _lasers_front (Variables|FaceParticles|GetLasers_Front))
  (bind _lasers_back (Variables|FaceParticles|GetLasers_Back))
  (bind _lasers_left (Variables|FaceParticles|GetLasers_Left))
  (bind _lasers_right (Variables|FaceParticles|GetLasers_Right))
  (bind _lasers_top (Variables|FaceParticles|GetLasers_Top))
  (bind _lasers_bottom (Variables|FaceParticles|GetLasers_Bottom))
  (bind _lasercomponents (Variables|Settings|GetLaserComponents))
  (bind _item (Utilities|Array|Get(acopy) _lasercomponents Array%20Index))
  (bind _returnvalue (Utilities|Select :Index Array%20Index :Option%200 _lasers_front :Option%201 _lasers_back :Option%202 _lasers_left :Option%203 _lasers_right :Option%204 _lasers_top :Option%205 _lasers_bottom))
  (if (Utilities|Array|IsValidIndex _returnvalue)
    (Default|FireLaser _item _item (Variables|/Game/Blueprints/Misc/Components/BP_CB_Raycast_Component_00.BP_CB_Raycast_Component_00_C|GetHeldColour (Variables|Default|GetBP_CB_Raycast_Component_00)) _returnvalue (Variables|PassThroughVariables|GetMaxBounce) (Variables|PassThroughVariables|GetInputPower))))

(fn RefractD
  (params (Array%20Index :type Integer%20%28by%20ref%29))
  (bind _lasers_front (Variables|FaceParticles|GetLasers_Front))
  (bind _lasers_back (Variables|FaceParticles|GetLasers_Back))
  (bind _lasers_left (Variables|FaceParticles|GetLasers_Left))
  (bind _lasers_right (Variables|FaceParticles|GetLasers_Right))
  (bind _lasers_top (Variables|FaceParticles|GetLasers_Top))
  (bind _lasers_bottom (Variables|FaceParticles|GetLasers_Bottom))
  (bind _lasercomponents (Variables|Settings|GetLaserComponents))
  (bind _frontdispersion (Variables|DispersionValues|GetFrontDispersion))
  (bind _backdispersion (Variables|DispersionValues|GetBackDispersion))
  (bind _leftdispersion (Variables|DispersionValues|GetLeftDispersion))
  (bind _rightdispersion (Variables|DispersionValues|GetRightDispersion))
  (bind _topdispersion (Variables|DispersionValues|GetTopDispersion))
  (bind _bottomdispersion (Variables|DispersionValues|GetBottomDispersion))
  (bind _item (Utilities|Array|Get(acopy) _lasercomponents Array%20Index))
  (bind _returnvalue (Utilities|Select :Index Array%20Index :Option%200 _lasers_front :Option%201 _lasers_back :Option%202 _lasers_left :Option%203 _lasers_right :Option%204 _lasers_top :Option%205 _lasers_bottom))
  (bind _returnvalue_2 (Utilities|Select :Index Array%20Index :Option%200 _frontdispersion :Option%201 _backdispersion :Option%202 _leftdispersion :Option%203 _rightdispersion :Option%204 _topdispersion :Option%205 _bottomdispersion))
  (if (and (Check|DispersionCheck _returnvalue_2) (Utilities|Array|IsValidIndex _returnvalue Array%20Index))
    (Default|FireLaser _item _item _returnvalue_2 _returnvalue (Variables|PassThroughVariables|GetMaxBounce) (Variables|PassThroughVariables|GetInputPower))))

(fn DispersionCheck
  (params (DispersionColour :type Linear%20Color%20Structure%20%28by%20ref%29))
  (bind _bp_cb_raycast_component_00 (Variables|Default|GetBP_CB_Raycast_Component_00))
  (bind _heldcolour (Variables|/Game/Blueprints/Misc/Components/BP_CB_Raycast_Component_00.BP_CB_Raycast_Component_00_C|GetHeldColour _bp_cb_raycast_component_00))
  (return (Math|Boolean|ANDBoolean (>= (.r _heldcolour) (.r DispersionColour)) (>= (.g _heldcolour) (.g DispersionColour)) (>= (.b _heldcolour) (.b DispersionColour)))))

(fn Possesion
  (bind _bp_cb_raycast_component_00 (Variables|Default|GetBP_CB_Raycast_Component_00))
  (bind _setobjectactive (Variables|/Game/Blueprints/Misc/Components/BP_CB_Raycast_Component_00.BP_CB_Raycast_Component_00_C|GetSetObjectActive _bp_cb_raycast_component_00))
  (if _setobjectactive
    (bind _asbp_cb_player_controller_00 (Utilities|Casting|CastToBP_CB_PlayerController_00 (Game|Player|GetPlayerPawn 0))
      (:then
        (bind _output_get (Variables|Default|SetPlayer%20Controller _asbp_cb_player_controller_00))
        (Default|TogglePossesion _output_get _setobjectactive self))
      (:CastFailed
        _)))
  (return _bp_cb_raycast_component_00))