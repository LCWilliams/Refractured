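; Moving platform that slides its mesh between StartPoint and EndPoint, optionally carrying an attached actor, for laser-receiver puzzles.
; A looping timeline, rate set by PerformanceDelay, acts as a throttled tick that checks receivers when NeedsPower is set, with StartsActive inverting the result.
; Once mode plays or reverses with that state, Back and Forth only starts its timeline, and Player mode arms box overlaps to drive movement.
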(event OnComponentBeginOverlap(Box)
  (params (OverlappedComponent :type Primitive%20Component%20Object%20Reference) (OtherActor :type Actor%20Object%20Reference) (OtherComp :type Primitive%20Component%20Object%20Reference) (OtherBodyIndex :type Integer) (bFromSweep :type Boolean) (SweepResult :type Hit%20Result%20Structure%20%28by%20ref%29))
  (if (and (== OtherActor (Game|Player|GetPlayerPawn 0)) (stale EventBeginPlay _output_get))
    (bind _platform (Timeline|Timeline_1 Play)
      (:Update
        (Transformation|SetRelativeLocation (Variables|Default|GetSM_MC_Platform_00) (Math|Vector|Lerp(Vector) (Variables|Config|GetStartPoint) (Variables|Config|GetEndPoint) _platform) false false)))))

(event OnComponentEndOverlap(Box)
  (params (OverlappedComponent :type Primitive%20Component%20Object%20Reference) (OtherActor :type Actor%20Object%20Reference) (OtherComp :type Primitive%20Component%20Object%20Reference) (OtherBodyIndex :type Integer))
  (if (and (stale EventBeginPlay _output_get) (== (Game|Player|GetPlayerPawn 0) OtherActor))
    (bind _platform (Timeline|Timeline_1 Reverse)
      (:Update
        (Transformation|SetRelativeLocation (Variables|Default|GetSM_MC_Platform_00) (Math|Vector|Lerp(Vector) (Variables|Config|GetStartPoint) (Variables|Config|GetEndPoint) _platform) false false)))))

(event EventBeginPlay
  (bind _attachedactor (Variables|Config|GetAttachedActor))
  (Utilities|FlowControl|Sequence
    (:then_0
      (Components|Timeline|SetPlayRate (Variables|Default|GetLooping) (Variables|Default|GetPerformanceDelay))
      (Timeline|Looping PlayFromStart
        (:NewTrack_1
          (if (Variables|Config|GetNeedsPower)
            (bind _returnvalue (CallFunction|CheckReceivers (Variables|Config|GetLaserRecieverRef))))
          (switch Utilities|FlowControl|Switch|SwitchonE_CB_PlatformMode_00 (Variables|Config|GetPlatfrom%20Mode)
            (:NewEnumerator0
              (if (select (Variables|Config|GetStartsActive) (not _returnvalue) _returnvalue)
                (bind _platform (Timeline|PlatformTimeLine Play)
                  (:Update
                    (Transformation|SetRelativeLocation (Variables|Default|GetSM_MC_Platform_00) (Math|Vector|Lerp(Vector) (Variables|Config|GetStartPoint) (Variables|Config|GetEndPoint) _platform) false false)))
                (else
                  (Timeline|PlatformTimeLine Reverse))))
            (:NewEnumerator1
              (if (select (Variables|Config|GetStartsActive) (not _returnvalue) _returnvalue)
                (bind _platform_2 (Timeline|Timeline_0 Play)
                  (:Update
                    (Transformation|SetRelativeLocation (Variables|Default|GetSM_MC_Platform_00) (Math|Vector|Lerp(Vector) (Variables|Config|GetStartPoint) (Variables|Config|GetEndPoint) _platform_2) false false)))))
            (:NewEnumerator2
              (if (select (Variables|Config|GetStartsActive) (not _returnvalue) _returnvalue)
                (bind _output_get (Variables|Config|SetHasAttatchedActor true))
                (else
                  (Variables|Config|SetHasAttatchedActor false))))))))
    (:then_1
      (Utilities|IsValid _attachedactor
        (:Is%20Valid
          (Transformation|AttachComponentToComponent _attachedactor (Variables|Default|GetSM_MC_Platform_00) "None" "KeepRelative" "KeepRelative" "KeepRelative" true))))))

(fn ConstructionScript)