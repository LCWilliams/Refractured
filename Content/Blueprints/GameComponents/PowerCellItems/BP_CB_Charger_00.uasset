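; BP_CB_Charger_00 is a single-use charger that adds charge to the player's power cell when activated while the player holds the power ball.
; Tick polls and clears the raycast component's activation flag, then a DoOnce applies the charge and completes an optional numbered objective.
; A timeline animates the UI battery bar from old to new charge, with the status showing charging until it returns to idle.
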(event EventTick
  (params (DeltaSeconds :type Float%20%28single-precision%29))
  (bind _player (Variables|Default|GetPlayer))
  (bind _gameuireference (Variables|/Game/Blueprints/GameComponents/Player/BP_CB_PlayerController_00.BP_CB_PlayerController_00_C|GetGameUIReference _player))
  ;[1 1 1] Increments the Power cell charge when activated
  (if (Variables|/Game/Blueprints/Misc/Components/BP_CB_Raycast_Component_00.BP_CB_Raycast_Component_00_C|GetSetObjectActive (Variables|Default|GetBP_CB_Raycast_Component_00))
    (Utilities|FlowControl|Delay 0.0001)
    (Variables|/Game/Blueprints/Misc/Components/BP_CB_Raycast_Component_00.BP_CB_Raycast_Component_00_C|SetSetObjectActive (Variables|Default|GetBP_CB_Raycast_Component_00) false)
    (if (Variables|/Game/Blueprints/GameComponents/Player/BP_CB_PlayerController_00.BP_CB_PlayerController_00_C|GethasPowerBall _player)
      (Utilities|FlowControl|DoOnce false
        (:Completed
          (CallFunction|UpdateObjective)
          (bind _output_get (Variables|Default|SetPowerCellChargePrior (Variables|/Game/Blueprints/GameComponents/Player/BP_CB_PlayerController_00.BP_CB_PlayerController_00_C|GetPowerCellCharge _player)))
          (bind _output_get_2 (Variables|/Game/Blueprints/GameComponents/Player/BP_CB_PlayerController_00.BP_CB_PlayerController_00_C|SetPowerCellCharge _player (+ (Variables|/Game/Blueprints/GameComponents/Player/BP_CB_PlayerController_00.BP_CB_PlayerController_00_C|GetPowerCellCharge _player) (Variables|Default|GetChargeAmount)))) ; Add battery icon update after this.
          (Default|StatusChangeCharging _gameuireference)
          (bind _lerptrack (Timeline|LerpValue Play)
            (:Update
              (Progress|SetPercent (Variables|/Game/Blueprints/GameComponents/Player/GraphicalUserInterface/BP_LW_GameHUD.BP_LW_GameHUD_C|GetBattery_Progress _gameuireference) (Math|Float|Lerp _output_get _output_get_2 _lerptrack)))
            (:Finished
              (Default|StatusChangeIdle _gameuireference))))))))

(event EventBeginPlay
  ;[1 1 1] Get Player
  (Variables|Default|SetPlayer (.AsBP%20CB%20Player%20Controller%2000 (Utilities|Casting|CastToBP_CB_PlayerController_00 (Game|Player|GetPlayerPawn 0)))))

(fn ConstructionScript)

(fn UpdateObjective
  (bind _objectivenumber (Variables|Default|GetObjectiveNumber))
  (if (Variables|Default|GetObjectiveCalled)
    _
    (elif (!= _objectivenumber -1)
      (Default|CompleteCurrentObjective (Variables|Default|GetPlayer) _objectivenumber)
      (Variables|Default|SetObjectiveCalled true)
      (return)
      (else
        _)))
  (return))