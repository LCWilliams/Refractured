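; Laser-activated switch that becomes active when a laser of its required colour hits it.
; On begin play it tints its cube with RequiredColour through a dynamic material instance.
; On overlap with a Laser-tagged component of a BP_CB_Laserhub_02b, CompareColours checks the hub's colour against RequiredColour to set IsActive.
; When overlap ends, it deactivates only if IsSwitch is false and the hub's colour matches black, so IsSwitch latches it on.
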(event OnComponentBeginOverlap(Cube)
  (params (OverlappedComponent :type Primitive%20Component%20Object%20Reference) (OtherActor :type Actor%20Object%20Reference) (OtherComp :type Primitive%20Component%20Object%20Reference) (OtherBodyIndex :type Integer) (bFromSweep :type Boolean) (SweepResult :type Hit%20Result%20Structure%20%28by%20ref%29))
  ;[1 1 1] Sets Active if compared colour are close to equal
  (if (not (Variables|Default|GetisActive))
    (bind _asbp_cb_laserhub_02b (Utilities|Casting|CastToBP_CB_Laserhub_02b OtherActor))
    (Variables|Default|SetisActive (and (Components|ComponentHasTag OtherComp "Laser") (CallFunction|CompareColours (Variables|/Game/Blueprints/BP_CB_Laserhub_02b.BP_CB_Laserhub_02b_C|GetLaserColour _asbp_cb_laserhub_02b) (Variables|Default|GetRequiredColour))))))

(event OnComponentEndOverlap(Cube)
  (params (OverlappedComponent :type Primitive%20Component%20Object%20Reference) (OtherActor :type Actor%20Object%20Reference) (OtherComp :type Primitive%20Component%20Object%20Reference) (OtherBodyIndex :type Integer))
  ;[1 1 1] Sets Active if compared colour are close to equal
  ;;[1 1 1] Sets Not Active if Colours are close to equal
  (if (not (Variables|Default|GetisSwitch))
    (bind _asbp_cb_laserhub_02b (Utilities|Casting|CastToBP_CB_Laserhub_02b OtherActor))
    (if (CallFunction|CompareColours (Variables|/Game/Blueprints/BP_CB_Laserhub_02b.BP_CB_Laserhub_02b_C|GetLaserColour _asbp_cb_laserhub_02b))
      (Variables|Default|SetisActive false))))

(event Collision|EventActorBeginOverlap
  (params (OtherActor :type Actor%20Object%20Reference)))

(event EventTick
  (params (DeltaSeconds :type Float%20%28single-precision%29)))

(event EventBeginPlay
  (bind _cube (Variables|Default|GetCube))
  ;[1 1 1] Set switch colour
  (bind _returnvalue (Rendering|Material|CreateDynamicMaterialInstance _cube 0 "/Game/Materials/M_LW_ActivatableComponent_00.M_LW_ActivatableComponent_00" :!class /Script/Engine.PrimitiveComponent))
  (Rendering|Material|SetMaterial _cube 0 _returnvalue)
  (Rendering|Material|SetVectorParameterValue _returnvalue "SwitchColour" (Variables|Default|GetRequiredColour) :!class /Script/Engine.MaterialInstanceDynamic))

(fn ConstructionScript
  (|CallParentFunction))