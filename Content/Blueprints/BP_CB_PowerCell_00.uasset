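; BP_CB_PowerCell_00 is the power cell objective at the elevator, which the player takes out and must bring back charged.
; Leaving the Box trigger gives the player the cell and hides the Cube.
; Re-entering compares the player's charge to TargetCharge, showing the Cube and printing "Level End" on success, or a warning otherwise.
; SetTargetCharge sets a new target and zeroes the player's charge.
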(event OnComponentEndOverlap(Box)
  (params (OverlappedComponent :type Primitive%20Component%20Object%20Reference) (OtherActor :type Actor%20Object%20Reference) (OtherComp :type Primitive%20Component%20Object%20Reference) (OtherBodyIndex :type Integer))
  (bind _player (Variables|Default|GetPlayer))
  ;[1 1 1] Player Picks up cell when leaving the Elevator
  (if (== OtherActor _player)
    (Variables|/Game/Blueprints/Player/BP_CB_PlayerController_00.BP_CB_PlayerController_00_C|SethasPowerBall _player true)
    (Rendering|SetVisibility (Variables|Default|GetCube) false false)
    (Development|PrintString "You have the power Cell")))

(event OnComponentBeginOverlap(Box)
  (params (OverlappedComponent :type Primitive%20Component%20Object%20Reference) (OtherActor :type Actor%20Object%20Reference) (OtherComp :type Primitive%20Component%20Object%20Reference) (OtherBodyIndex :type Integer) (bFromSweep :type Boolean) (SweepResult :type Hit%20Result%20Structure%20%28by%20ref%29))
  (bind _player (Variables|Default|GetPlayer))
  ;[1 1 1] Upon returning to the elevator, checks if the cell is charged enough
  (if (== OtherActor _player)
    (if (Variables|/Game/Blueprints/Player/BP_CB_PlayerController_00.BP_CB_PlayerController_00_C|GethasPowerBall _player)
      (if (>= (Variables|/Game/Blueprints/Player/BP_CB_PlayerController_00.BP_CB_PlayerController_00_C|GetPowerCellCharge _player) (Variables|Default|GetTargetCharge))
        (Rendering|SetVisibility (Variables|Default|GetCube) true false)
        (Development|PrintString "Level End")
        (else
          (Development|PrintString "Insufficient Charge")))
      (else
        (Development|PrintString "You don't have the power cell?")))))

(event Custom|Set%20Target%20Charge
  (params (TargetCharge :type Integer))
  ;[1 1 1] Event to reset Target Charge on level end
  (Variables|Default|SetTargetCharge TargetCharge)
  (Variables|/Game/Blueprints/Player/BP_CB_PlayerController_00.BP_CB_PlayerController_00_C|SetPowerCellCharge (Variables|Default|GetPlayer) 0))

(event EventBeginPlay
  ;[1 1 1] Get Player
  (bind _asbp_cb_player_controller_00 (Utilities|Casting|CastToBP_CB_PlayerController_00 (Game|Player|GetPlayerPawn 0)))
  (Variables|Default|SetPlayer _asbp_cb_player_controller_00))

(fn ConstructionScript)