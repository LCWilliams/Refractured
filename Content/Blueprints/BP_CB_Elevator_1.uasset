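; Elevator actor that acts as a keyboard-driven level selector for testing level streaming, with no movement logic.
; It enables player input on BeginPlay, and the Add and Subtract keys step a target level index with wraparound.
; NumPad Zero unloads the current streamed level, builds the new level name from a fixed prefix plus the index, and streams it in visible without blocking.
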(event EventBeginPlay
  ;[1 1 1] Allows Actor To receive Input
  (Input|EnableInput (Game|GetPlayerController 0)))

(event EventTick
  (params (DeltaSeconds :type Float%20%28single-precision%29))
  ;[1 1 1] Testing Selection
)

(event Input|KeyboardEvents|Subtract
  (params (Key :type Key%20Structure :default "AnyKey"))
  ;[1 1 1] Decrease Level Selection
  (:Pressed
    (if (> (Variables|Default|GetTarget%20Level) 0)
      (bind _output_get (Variables|Default|SetTarget%20Level (- (stale _output_get) 1)))
      (else
        (Variables|Default|SetTarget%20Level (Variables|Default|GetNoOfLevels))))))

(event Input|KeyboardEvents|Add
  (params (Key :type Key%20Structure :default "AnyKey"))
  ;[1 1 1] Increase Level Selection
  (:Released
    (if (< (Variables|Default|GetTarget%20Level) (Variables|Default|GetNoOfLevels))
      (bind _output_get (Variables|Default|SetTarget%20Level (+ (stale _output_get) 1)))
      (else
        (Variables|Default|SetTarget%20Level 0)))))

(event Input|KeyboardEvents|NumPadZero
  (params (Key :type Key%20Structure :default "AnyKey"))
  ;[1 1 1] Loads Selected Level
  (:Pressed
    (Game|UnloadStreamLevel(byName) (Variables|Default|GetCurrent%20Level))
    (bind _output_get (Variables|Default|SetCurrent%20Level (Utilities|String|StringToName (Utilities|String|BuildString(Integer) "L_CB_Test_levelStreming_0" "" (Variables|Default|GetTarget%20Level)))))
    (Game|LoadStreamLevel(byName) _output_get true)))

(fn ConstructionScript)