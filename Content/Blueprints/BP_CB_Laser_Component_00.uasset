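; Laser component that fires a bouncing line-trace beam to power laser switches with a colour.
; Each fire restarts from the laser's transform, continuing along impact normals (not mirrored) off reflective-tagged actors or components, up to a bounce limit.
; Only the first hit sets the visible particle beam's endpoint.
; A hit-check macro passes colour and active state to the cached switch's raycast component, using a DoOnce to deactivate it.
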(fn TraceSetup
  (params (Laser%20Transform :type Scene%20Component%20Object%20Reference))
  (Variables|Default|SetCanBounce true)
  (bind _output_get (Variables|Default|SetLaserTransform (Transformation|GetWorldTransform Laser%20Transform)))
  (bind _output_get_2 (Variables|Default|SetStartLocation (.Location (Math|Transform|BreakTransform _output_get))))
  (bind _output_get_3 (Variables|Default|SetStartDirection (Math|Vector|GetForwardVector Laser%20Transform)))
  (Variables|Default|SetRayLocation _output_get_2)
  (Variables|Default|SetRayDirection _output_get_3))

(fn TraceUpdate
  (params (LaserColour :type Linear%20Color%20Structure) (VisualLaser :type Particle%20System%20Component%20Object%20Reference))
  (bind _returnvalue (Game|GetGameMode))
  (bind _asbp_cb_gamemode_00 (Utilities|Casting|CastToBP_CB_Gamemode_00 _returnvalue))
  (bind _tag_reflective (Variables|/Game/Blueprints/BP_CB_Gamemode_00.BP_CB_Gamemode_00_C|GetTag_Reflective _asbp_cb_gamemode_00))
  (bind _output_get (Variables|Default|SetBounceCount 0))
  (while (and (Variables|Default|GetCanBounce) (< _output_get (Variables|Default|GetMaxBounce)))
    (bind (_outhit _returnvalue_2) (Collision|LineTraceByChannel (Variables|Default|GetRayLocation) (+ (Variables|Default|GetRayLocation) (* (Variables|Default|GetRayDirection) 10000)) "TraceTypeQuery1" false (LocalVariables|GetIgnoreActors) "ForOneFrame" true "(R=1.000000,G=0.000000,B=0.000000,A=1.000000)" "(R=0.000000,G=1.000000,B=0.000000,A=1.000000)" 0.001))
    (if _returnvalue_2
      (LocalVariables|SetIgnoreActors (Utilities|Array|MakeArray (.HitActor (Collision|BreakHitResult _outhit))))
      (bind _result (Math|Integer|IncrementInt (Variables|Default|GetBounceCount))
        (:%20%20
          (Variables|Default|SetBounceCount _result)
          (bind _output_get_2 (Variables|Default|SetRayLocation (.ImpactPoint (Collision|BreakHitResult _outhit))))
          (Variables|Default|SetRayDirection (.ImpactNormal (Collision|BreakHitResult _outhit)))
          (if (== (Variables|Default|GetBounceCount) 1)
            ;[1 1 1] This node for visual laser
            (Class|ParticleSystemComponent|SetBeamTargetPoint VisualLaser 0 _output_get_2)
            (Effects|Components|ParticleSystem|SetEmitterEnable VisualLaser "Beam" true))
          (Utilities|TraceHitCheckM (.HitActor (Collision|BreakHitResult _outhit)) LaserColour
            (:Out
              (if (not (or (Actor|ActorHasTag (.HitActor (Collision|BreakHitResult _outhit)) _tag_reflective) (Components|ComponentHasTag (.HitComponent (Collision|BreakHitResult _outhit)) _tag_reflective)))
                (Variables|Default|SetCanBounce false)
                (Variables|Default|SetLoopEnd false))))))
      (else
        (Variables|Default|SetCanBounce false)
        (Variables|Default|SetLoopEnd false)))))

(fn FireLaser
  (params (LaserTransformRef :type Scene%20Component%20Object%20Reference) (LaserColour :type Linear%20Color%20Structure) (VisualLaserRef :type Particle%20System%20Component%20Object%20Reference))
  (if (not (Variables|Default|GetLoopEnd))
    (CallFunction|TraceSetup LaserTransformRef)
    (CallFunction|TraceUpdate LaserColour VisualLaserRef)))