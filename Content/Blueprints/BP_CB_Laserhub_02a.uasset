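; Laser hub actor with a beam effect and a skeletal laser that the player can aim.
; Tick enables player input while its raycast component's SetObjectActive flag is set, and the Activate input clears it.
; Turn and LookUp rotate the body and head bones, though Turn resets its angle each call instead of accumulating.
; BeginPlay colours and disables the beam; the trace, reflection and target-activation logic is disconnected and never runs.
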(event EventTick
  (params (DeltaSeconds :type Float%20%28single-precision%29))
  (bind _returnvalue (Game|GetPlayerController 0))
  (Utilities|FlowControl|Sequence
    (:then_1
      (if (Variables|/Game/Blueprints/BP_CB_Raycast_Component_00.BP_CB_Raycast_Component_00_C|GetSetObjectActive (Variables|Default|GetBP_CB_Raycast_Component_00))
        (Input|EnableInput _returnvalue)
        (else
          (Input|DisableInput _returnvalue))))))

(event EventBeginPlay
  (bind _ps_lw_laserbeam_00 (Variables|Default|GetPS_LW_LaserBeam_00))
  (Effects|Components|ParticleSystem|SetColorParameter _ps_lw_laserbeam_00 "BeamColour" (Variables|Laser|GetLaserColour))
  (Effects|Components|ParticleSystem|SetEmitterEnable _ps_lw_laserbeam_00 "Beam" false)
  (Effects|Components|ParticleSystem|SetEmitterEnable _ps_lw_laserbeam_00 "BeamDischarge" false))

(event Input|ActionEvents|InputActionActivate
  (params (Key :type Key%20Structure :default "AnyKey"))
  (:Pressed
    (Variables|/Game/Blueprints/BP_CB_Raycast_Component_00.BP_CB_Raycast_Component_00_C|SetSetObjectActive (Variables|Default|GetBP_CB_Raycast_Component_00) false)))

(event Input|AxisEvents|InputAxisTurn
  (params (AxisValue :type Float%20%28single-precision%29))
  (bind _output_get (Variables|Default|SetCurrent%20Pitch 0.0))
  (Components|PoseableMesh|SetBoneRotationbyName (Variables|Default|GetSkM_LW_Laser_00_Laser) "LaserBody" (Math|Rotator|MakeRotator 0.0 (+ _output_get (* AxisValue (Variables|Rotation|GetRotation%20Speed) (Utilities|Time|GetWorldDeltaSeconds))) 0.0) "ComponentSpace"))

(event Input|AxisEvents|InputAxisLookUp
  (params (AxisValue :type Float%20%28single-precision%29))
  (bind _output_get (Variables|Default|SetCurrent%20Yaw (+ (stale _output_get) (* AxisValue (Variables|Rotation|GetRotation%20Speed) (Utilities|Time|GetWorldDeltaSeconds) -1.0))))
  (Components|PoseableMesh|SetBoneRotationbyName (Variables|Default|GetSkM_LW_Laser_00_Laser) "LaserHead" (Math|Rotator|MakeRotator 0.0 _output_get 0.0) "ComponentSpace"))

(fn ConstructionScript)