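; Shared function library for Refractured's laser puzzle mechanics, covering beam tracing, laser effects and interaction checks.
; A laser trace returns hit data, while helpers test actor or component tags for reflective, laser-activated, player-activated and grabbable objects, using names from CommonTags.
; Laser helpers spawn beam emitter arrays, toggle normal and high-power emitters, and collapse beams onto their owner.
; Other helpers identify interactable classes and set the first power cell's target charge.
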(fn CommonTags
  (return "Reflective" "PlayerActivatable" "LaserActivatable" "Grab"))

(fn FireLaserLinetrace
  (params (LaserPointStart :type Vector%20%28by%20ref%29) (LaserPointDirection :type Vector%20%28by%20ref%29) (Laser%20Length :type Integer) (Actors%20To%20Ignore :type Array%20of%20Actor%20Object%20References))
  (bind (_outhit _returnvalue) (Collision|LineTraceByChannel 0 LaserPointStart (+ LaserPointStart (* LaserPointDirection Laser%20Length)) "TraceTypeQuery1" false Actors%20To%20Ignore "None" true "(R=1.000000,G=0.000000,B=0.000000,A=1.000000)" "(R=0.000000,G=1.000000,B=0.000000,A=1.000000)" 1.0))
  (if _returnvalue
    _
    (else
      _))
  (return _returnvalue (.Location (Collision|BreakHitResult _outhit)) (.ImpactNormal (Collision|BreakHitResult _outhit)) LaserPointStart (Utilities|Array|MakeArray (.HitActor (Collision|BreakHitResult _outhit))) (.HitActor (Collision|BreakHitResult _outhit)) (.HitComponent (Collision|BreakHitResult _outhit))))

(fn CheckReflectivity
  (params (Hit%20Actor :type Actor%20Object%20Reference%20%28by%20ref%29) (Hit%20Actor%20Component :type Primitive%20Component%20Object%20Reference))
  (bind _reflective (Check|CommonTags))
  (return (or (Actor|ActorHasTag Hit%20Actor _reflective) (Components|ComponentHasTag Hit%20Actor%20Component _reflective))))

(fn InstantiateLasers
  (params (Ammount%20to%20Instantiate :type Integer%20%28by%20ref%29) (LaserParticleSystemTemplate :type Particle%20System%20Object%20Reference) (Ignore%20First :type Boolean) (Location :type Vector))
  (bind _laserarray (LocalVariables|GetLaserArray))
  (if Ignore%20First ; Ignore first: Used if there is a pre-existing first particle.
    (for _index (range 2 Ammount%20to%20Instantiate)
      (bind _returnvalue (Effects|SpawnEmitteratLocation 0 LaserParticleSystemTemplate Location "0, 0, 0" false))
      (Utilities|Array|Add _laserarray _returnvalue)
      (Utilities|ChangeLaserState _laserarray false false false) ; Disable lasers on spawn.
    )
    (else
      (for _index_2 (range 1 Ammount%20to%20Instantiate)
        (bind _returnvalue_2 (Effects|SpawnEmitteratLocation 0 LaserParticleSystemTemplate Location "0, 0, 0" false))
        (Utilities|Array|Add _laserarray _returnvalue_2)
        (Utilities|ChangeLaserState _laserarray false false false) ; Disable lasers on spawn.
      )))
  (return _laserarray))

(fn LaserActivated
  (params (Hit%20Actor :type Actor%20Object%20Reference%20%28by%20ref%29) (Hit%20Actor%20Component :type Primitive%20Component%20Object%20Reference))
  (bind _activated_by_laser (Check|CommonTags))
  (bind _returnvalue (Actor|ActorHasTag Hit%20Actor _activated_by_laser))
  (Utilities|IsValid Hit%20Actor%20Component
    (:Is%20Valid
      (return (or (Components|ComponentHasTag Hit%20Actor%20Component _activated_by_laser) _returnvalue)))
    (:Is%20Not%20Valid
      (return _returnvalue))))

(fn PlayerActivated
  (params (Hit%20Actor :type Actor%20Object%20Reference%20%28by%20ref%29) (Hit%20Actor%20Component :type Primitive%20Component%20Object%20Reference))
  (bind _activated_by_player (Check|CommonTags))
  (bind _returnvalue (Actor|ActorHasTag Hit%20Actor _activated_by_player))
  (Utilities|IsValid Hit%20Actor%20Component
    (:Is%20Valid
      (return (or (Components|ComponentHasTag Hit%20Actor%20Component _activated_by_player) _returnvalue)))
    (:Is%20Not%20Valid
      (return _returnvalue))))

(fn LaserElements
  (params (Raycast%20Component :type BP%20CB%20Raycast%20Component%2000%20Object%20Reference%20%28by%20ref%29))
  (return (Variables|/Game/Blueprints/Misc/Components/BP_CB_Raycast_Component_00.BP_CB_Raycast_Component_00_C|GetSentPower Raycast%20Component) (Variables|/Game/Blueprints/Misc/Components/BP_CB_Raycast_Component_00.BP_CB_Raycast_Component_00_C|GetSentColour Raycast%20Component)))

(fn ResetLaserPosition
  (params (Laser%20Array :type Array%20of%20Particle%20System%20Component%20Object%20References) (SelfReference :type Actor%20Object%20Reference))
  (bind _returnvalue (Transformation|GetActorLocation SelfReference))
  (if (Utilities|Array|IsValidIndex Laser%20Array)
    (for _array_element Laser%20Array
      (Effects|Components|ParticleSystem|SetVectorParameter _array_element "BeamSource" _returnvalue)
      (Effects|Components|ParticleSystem|SetVectorParameter _array_element "BeamTarget" _returnvalue)
      (Effects|Components|ParticleSystem|SetVectorParameter _array_element "HPBeamSource" _returnvalue)
      (Effects|Components|ParticleSystem|SetVectorParameter _array_element "HPBeamTarget" _returnvalue)
      (Components|Activation|SetActive _array_element false true))))

(fn LaserArrayHasElements
  (params (Laser%20Array :type Array%20of%20Particle%20System%20Component%20Object%20References))
  (return (Utilities|IsValid (Utilities|Array|Get(acopy) Laser%20Array))))

(fn ResetLevelCharge
  (params (TargetCharge :type Float%20%28single-precision%29))
  (bind _outactors (Actor|GetAllActorsOfClass 0 "/Game/Blueprints/GameComponents/PowerCellItems/BP_CB_PowerCell_00.BP_CB_PowerCell_00_C"))
  (Default|SetTargetCharge (Utilities|Array|Get(acopy) _outactors) TargetCharge))

(fn Grabable
  (params (Hit%20Actor :type Actor%20Object%20Reference%20%28by%20ref%29) (Hit%20Actor%20Component :type Primitive%20Component%20Object%20Reference))
  (bind _grabable (Check|CommonTags))
  (bind _returnvalue (Actor|ActorHasTag Hit%20Actor _grabable))
  (Utilities|IsValid Hit%20Actor%20Component
    (:Is%20Valid
      (return (or _returnvalue (Components|ComponentHasTag Hit%20Actor%20Component _grabable))))
    (:Is%20Not%20Valid
      (return _returnvalue))))

(fn ChangeLaserState
  (params (Laser%20Array :type Array%20of%20Particle%20System%20Component%20Object%20References) (Enable :type Boolean) (OnlyHighPower :type Boolean) (OnlyLowPower :type Boolean))
  (if (Utilities|Array|IsValidIndex Laser%20Array)
    (for _array_element Laser%20Array
      (if OnlyHighPower
        (Effects|Components|ParticleSystem|SetEmitterEnable _array_element "HighPWRBeam" Enable :!label _label)
        (else
          (Effects|Components|ParticleSystem|SetEmitterEnable _array_element "NormalBeam" Enable)
          (if (not OnlyLowPower)
            (goto _label)))))))

(fn PlayerInteractableObject
  (params (Object%20to%20check :type Object%20Object%20Reference))
  (bind _returnvalue (Utilities|GetClass Object%20to%20check))
  (return (Math|Boolean|ORBoolean (Utilities|ClassIsChildOf _returnvalue "/Game/Blueprints/GameComponents/Switches/BP_CB_Switch_00.BP_CB_Switch_00_C") (Utilities|ClassIsChildOf _returnvalue "/Game/Blueprints/GameComponents/Lasers+Cubes/BP_CB_Laserhub_02c.BP_CB_Laserhub_02c_C") (Utilities|ClassIsChildOf _returnvalue "/Game/Blueprints/GameComponents/Lasers+Cubes/BP_CB_Cube_01.BP_CB_Cube_01_C") (Utilities|ClassIsChildOf _returnvalue "/Game/Blueprints/GameComponents/PowerCellItems/BP_CB_Charger_00.BP_CB_Charger_00_C"))))