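; Laser component that fires a coloured, bouncing beam to power puzzle objects and repel the player.
; FireLaser line-traces from each impact along the returned normal until a miss, non-reflective hit or bounce limit, drawing one particle beam per segment.
; Hit checks pass colour and power to the target's raycast component and deactivate the previous target; high-power beams knock the player back.
; Unused beam segments collapse to the component's location.
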(fn TraceSetup
  (params (Laser%20Transform :type Scene%20Component%20Object%20Reference))
  (Variables|Default|SetCanBounce true)
  (bind _output_get (Variables|Transforms|SetLaserTransform (Transformation|GetWorldTransform Laser%20Transform)))
  (bind _output_get_2 (Variables|Transforms|SetStartLocation (.Location (Math|Transform|BreakTransform _output_get))))
  (bind _output_get_3 (Variables|Transforms|SetStartDirection (Math|Vector|GetForwardVector Laser%20Transform)))
  (Variables|Transforms|SetRayLocation _output_get_2)
  (Variables|Transforms|SetRayDirection _output_get_3))

(fn TraceUpdate
  (params (LaserColour :type Linear%20Color%20Structure) (VisualLaser :type Array%20of%20Particle%20System%20Component%20Object%20References) (MaxBounces :type Integer) (LaserPower :type Integer))
  (bind _output_get (Variables|Default|SetBounceCount 0))
  (while (and (Variables|Default|GetCanBounce) (< _output_get MaxBounces))
    (bind (_has_hit_object _impact_point _impact_normal _laser_start_point _ignore_actors _actor_hit_by_line _actor_component_hit) (CallFunction|FireLaserLinetrace (Variables|Transforms|GetRayLocation) (Variables|Transforms|GetRayDirection) 50000 (LocalVariables|GetIgnoreActors)))
    (if _has_hit_object
      (LocalVariables|SetIgnoreActors _ignore_actors)
      (bind _result (Math|Integer|IncrementInt (stale _output_get_2))
        (:%20%20
          (bind _output_get_2 (Variables|Default|SetBounceCount _result))
          (bind _output_get_3 (Variables|Transforms|SetRayLocation _impact_point))
          (Variables|Transforms|SetRayDirection _impact_normal)
          (Components|Activation|SetActive (Utilities|Array|Get(acopy) VisualLaser (- _output_get_2 1)) true false)
          (Updates|UpdateLaserPositions VisualLaser (Variables|Default|GetBounceCount) _laser_start_point _output_get_3)
          (Utilities|TraceHitCheckM _actor_hit_by_line _actor_component_hit LaserPower LaserColour
            (:Out
              (Updates|UpdateLaserPosifNoBounce (Variables|Default|GetBounceCount) MaxBounces VisualLaser)
              (Variables|Default|SetLoopEnd false)))))
      (else
        (Variables|Default|SetCanBounce false)))))

(fn FireLaser
  (params (LaserTransformRef :type Scene%20Component%20Object%20Reference%20%28by%20ref%29) (LaserColour :type Linear%20Color%20Structure%20%28by%20ref%29) (VisualLaserRef :type Array%20of%20Particle%20System%20Component%20Object%20References) (MaxBounces :type Integer%20%28by%20ref%29) (LaserPower :type Integer))
  (for _array_element VisualLaserRef
    (Effects|Components|ParticleSystem|SetColorParameter _array_element "BeamColour" LaserColour)
    (bind _output_get (Variables|Default|SetHighPowerLaser (== LaserPower 1))))
  (if (not (Variables|Default|GetLoopEnd))
    (Setup|TraceSetup LaserTransformRef)
    ;[1 1 1] Ensures only the required emitters are enabled.
    (if _output_get
      (CallFunction|ChangeLaserState VisualLaserRef true false false)
      (else
        (CallFunction|ChangeLaserState VisualLaserRef true false true)))
    (Updates|TraceUpdate LaserColour VisualLaserRef MaxBounces LaserPower)))

(fn UpdateLaserPositions
  (params (ParticleArray :type Array%20of%20Particle%20System%20Component%20Object%20References) (ArrayIndex :type Integer%20%28by%20ref%29) (StartPosition :type Vector%20%28by%20ref%29) (EndPosition :type Vector%20%28by%20ref%29))
  (bind _returnvalue (- ArrayIndex 1))
  (bind _item (Utilities|Array|Get(acopy) ParticleArray _returnvalue))
  (Effects|Components|ParticleSystem|SetVectorParameter _item "BeamSource" StartPosition)
  (Effects|Components|ParticleSystem|SetVectorParameter _item "BeamTarget" EndPosition)
  ;[1 1 1] Update High Power Laser
  (if (Variables|Default|GetHighPowerLaser)
    (Effects|Components|ParticleSystem|SetVectorParameter _item "HPBeamSource" StartPosition)
    (Effects|Components|ParticleSystem|SetVectorParameter _item "HPBeamTarget" EndPosition)))

(fn UpdateLaserPosifNoBounce
  (params (CurrentBounce :type Integer) (MaximumBounces :type Integer%20%28by%20ref%29) (Particle%20Array :type Array%20of%20Particle%20System%20Component%20Object%20References))
  (bind _self self)
  (bind _returnvalue (Transformation|GetWorldLocation _self))
  (if (or (> CurrentBounce 1) (!= CurrentBounce MaximumBounces))
    (bind _result (Math|Integer|DecrementInt MaximumBounces)
      (:%20%20
        (for _index (range CurrentBounce _result)
          (Effects|Components|ParticleSystem|SetVectorParameter (Utilities|Array|Get(acopy) Particle%20Array _index) "BeamSource" _returnvalue)
          (Effects|Components|ParticleSystem|SetVectorParameter (Utilities|Array|Get(acopy) Particle%20Array _index) "BeamTarget" _returnvalue)
          (Effects|Components|ParticleSystem|SetVectorParameter (Utilities|Array|Get(acopy) Particle%20Array _index) "HPBeamSource" _returnvalue)
          (Effects|Components|ParticleSystem|SetVectorParameter (Utilities|Array|Get(acopy) Particle%20Array _index) "HPBeamTarget" _returnvalue))))))

(fn DisableLasers
  (params (Particle%20Array :type Array%20of%20Particle%20System%20Component%20Object%20References))
  (bind _self self)
  (bind _returnvalue (Transformation|GetWorldLocation _self))
  (if (Utilities|Array|IsValidIndex Particle%20Array)
    (for _array_element Particle%20Array
      (Effects|Components|ParticleSystem|SetVectorParameter _array_element "BeamSource" _returnvalue)
      (Effects|Components|ParticleSystem|SetVectorParameter _array_element "BeamTarget" _returnvalue)
      (Effects|Components|ParticleSystem|SetVectorParameter _array_element "HPBeamSource" _returnvalue)
      (Effects|Components|ParticleSystem|SetVectorParameter _array_element "HPBeamTarget" _returnvalue))))