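; Raycast component that receives a colour and power input and holds a toggleable active flag for its object.
; Dothething switches the input on, then uses a 0.001s retriggerable delay to switch it off once calls stop arriving, so repeated hits act as a held signal.
; InputActive uses DoOnce gates to limit repeat updates to the input count and the stored colour and power.
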(event Custom|InputActive
  (params (isEnabled :type Boolean) (Colour :type Linear%20Color%20Structure) (Power :type Integer))
  (if isEnabled
    (Utilities|FlowControl|Sequence
      (:then_0
        (goto _label Reset))
      (:then_1
        (goto _label_2 Reset)))
    (else
      (Utilities|FlowControl|Sequence
        (:then_0
          (Utilities|FlowControl|DoOnce true :!label _label
            (:Completed
              (bind _result (Math|Integer|DecrementInt (Variables|Default|GetInputAmount))
                (:%20%20
                  (Variables|Default|SetInputAmount _result)
                  (Variables|Default|SetSentColour "")
                  (Variables|Default|SetSentPower 0))))))
        (:then_1
          (Utilities|FlowControl|DoOnce false :!label _label_2
            (:Completed
              (bind _result_2 (Math|Integer|IncrementInt (Variables|Default|GetInputAmount))
                (:%20%20
                  (Variables|Default|SetInputAmount _result_2)
                  (Variables|Default|SetSentColour Colour)
                  (Variables|Default|SetSentPower Power))))))))))

(event Custom|Do%20the%20thing
  (params (Colour :type Linear%20Color%20Structure%20%28by%20ref%29) (Power :type Integer%20%28by%20ref%29))
  (CallFunction|InputActive true Colour Power)
  (Utilities|FlowControl|RetriggerableDelay 0.001)
  (CallFunction|InputActive false))

(event Custom|Toggle%20Active
  ;[1 0.4312 0.2477] Single switch
  (if (Variables|Default|GetSetObjectActive)
    (Variables|Default|SetSetObjectActive false)
    (else
      (Variables|Default|SetSetObjectActive true))))