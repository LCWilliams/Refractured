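; BP_SA_Laserhub_01 is a laser emitter that fires a straight beam while its activatable component's SetObjectActive flag is on.
; Each Tick it line traces on the Visibility channel along the Arrow component's forward vector, with debug drawing showing the beam.
; A single-bounce reflection off actors tagged "Reflective", using a mirrored-vector second trace, is present but not connected, so it never runs.
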(event EventTick
  (params (DeltaSeconds :type Float%20%28single-precision%29))
  (bind _arrow (Variables|Default|GetArrow))
  (bind _returnvalue (Transformation|GetWorldLocation _arrow))
  ;[1 1 1] Standard Raycast
  (if (Variables|/Game/Blueprints/BP_CB_Activatable_Component_00.BP_CB_Activatable_Component_00_C|GetSetObjectActive (Variables|Default|GetBP_CB_Activatable_Component_00))
    (bind _outhit (Collision|LineTraceByChannel _returnvalue (+ _returnvalue (* (Math|Vector|GetForwardVector (Transformation|GetWorldRotation _arrow)) 1e+04)) "TraceTypeQuery1" false 0 "ForDuration" true "(R=1.000000,G=0.000000,B=0.000000,A=1.000000)" "(R=0.000000,G=0.016063,B=1.000000,A=1.000000)" 0.1))))

(fn ConstructionScript)