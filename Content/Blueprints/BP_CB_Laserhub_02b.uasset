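; Possessable laser turret that fires a coloured beam to trigger LaserActivatable actors, optionally only while its power receiver is active.
; Turn and LookUp rotate body and head bones, with the socket driving camera and trace arrow each Tick.
; A line trace places the beam end and sends colour to raycast components, with a mirrored second trace bouncing once off Reflective hits.
; The raycast component's flag triggers possession; Activate returns control.
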(event EventTick
  (params (DeltaSeconds :type Float%20%28single-precision%29))
  (bind _ps_lw_laserbeam_00 (Variables|Default|GetPS_LW_LaserBeam_00))
  (bind _lasercollsion (Variables|Default|GetLaserCollsion))
  (bind _skm_lw_laser_01_laserbase (Variables|Default|GetSkM_LW_Laser_01_LaserBase))
  (bind _lasercollsion_2 (Variables|Default|GetLaserCollsion))
  (bind _arrow (Variables|Default|GetArrow))
  (bind _returnvalue (Transformation|GetWorldLocation _arrow))
  (bind _returnvalue_2 (Transformation|GetWorldRotation _arrow))
  (bind _returnvalue_3 (Transformation|GetSocketRotation _skm_lw_laser_01_laserbase "Socket_LaserOrigin"))
  (bind _returnvalue_4 (Math|Vector|GetForwardVector _returnvalue_2))
  (bind _returnvalue_5 (* _returnvalue_4 1e+04))
  (bind _returnvalue_6 (+ _returnvalue _returnvalue_5))
  (Utilities|FlowControl|Sequence
    (:then_0
      (Transformation|SetRelativeRotation (Variables|Default|GetCamera) _returnvalue_3 false false)
      (Transformation|SetRelativeRotation _arrow _returnvalue_3 false false)
      ;[1 1 1] First Raycast
      (if (Variables|Activation|GetNeedsPower)
        (if (Variables|/Game/Blueprints/BP_CB_LaserReciever_00.BP_CB_LaserReciever_00_C|GetisActive (Variables|Activation|GetReceiverRef))
          (bind _outhit (Collision|LineTraceByChannel _returnvalue _returnvalue_6 "TraceTypeQuery1" false 0 "ForOneFrame" true "(R=1.000000,G=0.000000,B=0.000000,A=1.000000)" "(R=0.000000,G=0.016063,B=1.000000,A=1.000000)" 0.1 :!label _label))
          (Transformation|SetWorldLocation _lasercollsion_2 (.ImpactPoint (Collision|BreakHitResult _outhit)) false true)
          (Class|ParticleSystemComponent|SetBeamTargetPoint _ps_lw_laserbeam_00 0 (.ImpactPoint (Collision|BreakHitResult _outhit)))
          (Effects|Components|ParticleSystem|SetEmitterEnable _ps_lw_laserbeam_00 "Beam" true)
          (if (Actor|ActorHasTag (.HitActor (Collision|BreakHitResult _outhit)) "LaserActivatable")
            (Default|SendColour (Actor|GetComponentbyClass (.HitActor (Collision|BreakHitResult _outhit)) "/Game/Blueprints/BP_CB_Raycast_Component_00.BP_CB_Raycast_Component_00_C") (Variables|Laser|GetLaserColour))
            (Components|Activation|Activate _lasercollsion_2 false)
            (else
              (Transformation|SetRelativeLocation _lasercollsion_2 "0, 0, 0" false true)
              ;[1 1 1] Reflection
              (Components|Activation|Deactivate _lasercollsion_2)))
          (if (or (Actor|ActorHasTag (.HitActor (Collision|BreakHitResult _outhit)) "Reflective") (Components|ComponentHasTag (.HitComponent (Collision|BreakHitResult _outhit)) "Reflective"))
            (bind _outhit_2 (Collision|LineTraceByChannel (+ (.ImpactPoint (Collision|BreakHitResult _outhit)) (.Normal (Collision|BreakHitResult _outhit))) (+ (.ImpactPoint (Collision|BreakHitResult _outhit)) (Math|Vector|MirrorVectorbyNormal (- _returnvalue_6 _returnvalue) (.ImpactNormal (Collision|BreakHitResult _outhit)))) "TraceTypeQuery1" false 0 "ForDuration" true "(R=1.000000,G=0.000000,B=0.000000,A=1.000000)" "(R=0.000000,G=0.039124,B=1.000000,A=1.000000)" 0.1))
            (if (Actor|ActorHasTag (.HitActor (Collision|BreakHitResult _outhit_2)) "LaserActivatable")
              (Default|SendColour (Actor|GetComponentbyClass (.HitActor (Collision|BreakHitResult _outhit_2)) "/Game/Blueprints/BP_CB_Raycast_Component_00.BP_CB_Raycast_Component_00_C") (Variables|Laser|GetLaserColour))))
          (else
            (Transformation|SetRelativeLocation _lasercollsion "0, 0, 0" false true)
            (Components|Activation|Deactivate _lasercollsion)
            (Effects|Components|ParticleSystem|SetEmitterEnable _ps_lw_laserbeam_00 "Beam" false)
            (Components|Activation|Activate _lasercollsion_2 false)))
        (else
          (goto _label))))
    (:then_1
      ;[1 1 1] Laser Pawn Possession
      (bind _bp_cb_raycast_component_00 (CallFunction|Possession)))))

(event EventBeginPlay
  (bind _ps_lw_laserbeam_00 (Variables|Default|GetPS_LW_LaserBeam_00))
  (Effects|Components|ParticleSystem|SetColorParameter _ps_lw_laserbeam_00 "BeamColour" (Variables|Laser|GetLaserColour))
  (Effects|Components|ParticleSystem|SetEmitterEnable _ps_lw_laserbeam_00 "Beam" false)
  (Components|Activation|Activate (Variables|Default|GetLaserCollsion) false))

(event Input|ActionEvents|InputActionActivate
  (params (Key :type Key%20Structure :default "AnyKey"))
  (bind _returnvalue (Game|GetPlayerController 0))
  ;[1 1 1] Laser Pawn Possession
  (:Pressed
    (Variables|/Game/Blueprints/BP_CB_Raycast_Component_00.BP_CB_Raycast_Component_00_C|SetSetObjectActive (stale EventTick _bp_cb_raycast_component_00) false)
    (Pawn|UnPossess _returnvalue)
    (Pawn|Possess _returnvalue (Variables|Default|GetPlayer%20Controller))))

(event Input|AxisEvents|InputAxisTurn
  (params (AxisValue :type Float%20%28single-precision%29))
  ;[1 1 1] Laser Rotation
  (bind _output_get (CallFunction|RotationYaw AxisValue (Variables|Rotation|GetZ-Speed) (Utilities|Time|GetWorldDeltaSeconds) (Variables|Default|GetSkM_LW_Laser_01_LaserBase))))

(event Input|AxisEvents|InputAxisLookUp
  (params (AxisValue :type Float%20%28single-precision%29))
  ;[1 1 1] Laser Rotation
  (CallFunction|RotationPitch (stale Input|AxisEvents|InputAxisTurn _output_get) AxisValue (Variables|Rotation|GetX-Speed) (Utilities|Time|GetWorldDeltaSeconds) (Variables|Default|GetSkM_LW_Laser_01_LaserBase)))

(fn ConstructionScript)

(fn Possession
  (bind _bp_cb_raycast_component_00 (Variables|Default|GetBP_CB_Raycast_Component_00))
  (bind _setobjectactive (Variables|/Game/Blueprints/BP_CB_Raycast_Component_00.BP_CB_Raycast_Component_00_C|GetSetObjectActive _bp_cb_raycast_component_00))
  (if _setobjectactive
    (bind _asbp_cb_player_controller_00 (Utilities|Casting|CastToBP_CB_PlayerController_00 (Game|Player|GetPlayerPawn 0)))
    (bind _output_get (Variables|Default|SetPlayer%20Controller _asbp_cb_player_controller_00))
    (Default|TogglePossesion _output_get _setobjectactive self)
    (return _bp_cb_raycast_component_00)))

(fn RotationYaw
  (params (InputAxis :type Float%20%28single-precision%29) (RotationSpeedModifier :type Float%20%28single-precision%29) (DeltaSeconds :type Float%20%28single-precision%29) (SkelatalMesh :type Poseable%20Mesh%20Component%20Object%20Reference))
  (bind _output_get (Variables|Rotation|SetCurrent%20Yaw (+ (stale _output_get) (* InputAxis RotationSpeedModifier DeltaSeconds))))
  (Components|PoseableMesh|SetBoneRotationbyName SkelatalMesh "LaserBody" (Math|Rotator|MakeRotator 9e+01 0.0 _output_get) "ComponentSpace")
  (return _output_get))

(fn RotationPitch
  (params (RotationYaw :type Float%20%28single-precision%29) (InputAxis :type Float%20%28single-precision%29) (RotationSpeedModifier :type Float%20%28single-precision%29) (DeltaSeconds :type Float%20%28single-precision%29) (SkelatalMesh :type Poseable%20Mesh%20Component%20Object%20Reference))
  (bind _output_get (Variables|Rotation|SetCurrent%20Pitch (+ (stale _output_get) (* InputAxis RotationSpeedModifier DeltaSeconds -1.0))))
  (bind _output_get_2 (Variables|Rotation|SetCurrent%20Pitch (Math|Float|Clamp(Float) _output_get 1.5e+02 2.4e+02)))
  (Components|PoseableMesh|SetBoneRotationbyName SkelatalMesh "LaserHead" (Math|Rotator|MakeRotator _output_get_2 1.8e+02 RotationYaw) "ComponentSpace"))