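; BP_CB_Switch_00 is a switch actor that turns active through a raycast component and plays a sound when it does.
; Each Tick copies the component's SetObjectActive flag into IsActive.
; A DoOnce gate limits the audio to one play per activation and resets whenever the switch is inactive.
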(event EventBeginPlay
  (|CallParentFunction))

(event Collision|EventActorBeginOverlap
  (params (OtherActor :type Actor%20Object%20Reference)))

(event EventTick
  (params (DeltaSeconds :type Float%20%28single-precision%29))
  ;[1 1 1] Toggles On Raycast
  (bind _output_get (Variables|Default|SetisActive (Variables|/Game/Blueprints/UnicornCube/BP_CB_Raycast_Component_00.BP_CB_Raycast_Component_00_C|GetSetObjectActive (Variables|Default|GetBP_CB_Raycast_Component_00))))
  (if _output_get
    (Utilities|FlowControl|DoOnce true :!label _label
      (:Completed
        (Audio|Components|Audio|Play (Variables|Default|GetAudio) 0.0)))
    (else
      (goto _label Reset))))

(fn ConstructionScript
  (|CallParentFunction))