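; Spline actor that lays a glowing static mesh along an editable spline, with configurable colour and emissive strength.
; The construction script adds one spline mesh component per segment, matching point positions and tangents, with query-only collision.
; All segments share a dynamic instance of an emissive master material.
; Colour and Strength are pushed to that material at construction, at BeginPlay and again every Tick.
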(event EventBeginPlay
  (bind _dynamicmaterial (Variables|Default|GetDynamicMaterial))
  (Rendering|Material|SetVectorParameterValue _dynamicmaterial "Colour" (Variables|Default|GetSplineColour) :!class /Script/Engine.MaterialInstanceDynamic)
  (Rendering|Material|SetScalarParameterValue _dynamicmaterial "Strength" (Variables|Default|GetStrength) :!class /Script/Engine.MaterialInstanceDynamic))

(event Collision|EventActorBeginOverlap
  (params (OtherActor :type Actor%20Object%20Reference)))

(event EventTick
  (params (DeltaSeconds :type Float%20%28single-precision%29))
  (bind _dynamicmaterial (Variables|Default|GetDynamicMaterial))
  (Rendering|Material|SetVectorParameterValue _dynamicmaterial "Colour" (Variables|Default|GetSplineColour) :!class /Script/Engine.MaterialInstanceDynamic)
  (Rendering|Material|SetScalarParameterValue _dynamicmaterial "Strength" (Variables|Default|GetStrength) :!class /Script/Engine.MaterialInstanceDynamic))

(fn ConstructionScript
  (bind _spline (Variables|Default|GetSpline))
  (bind _returnvalue (Rendering|Material|CreateDynamicMaterialInstance "/Game/Materials/Effects/Emissive/M_LW_BasicEmissive_Master.M_LW_BasicEmissive_Master" :!class /Script/Engine.KismetMaterialLibrary))
  (Variables|Default|SetDynamicMaterial _returnvalue)
  (for _index (range 0 (- (Spline|GetNumberOfSplinePoints _spline) 2))
    (bind _returnvalue_2 (AddComponent|AddSplineMeshComponent true))
    (bind _output_get (Variables|Default|SetSplineMesh _returnvalue_2))
    (Components|StaticMesh|SetStaticMesh _output_get (Variables|Default|GetStaticMesh))
    (SplineMesh|SetForwardAxis _returnvalue_2 (Variables|Default|GetForwardAxis) true)
    (Transformation|AttachComponentToComponent _returnvalue_2 _spline "None" "KeepRelative" "KeepRelative" "KeepRelative" true)
    (SplineMesh|SetStartandEnd _returnvalue_2 (Spline|GetLocationatSplinePoint _spline _index "Local") (Spline|GetTangentatSplinePoint _spline _index "Local") (Spline|GetLocationatSplinePoint _spline (+ _index 1) "Local") (Spline|GetTangentatSplinePoint _spline (+ _index 1) "Local") true :!class /Script/Engine.SplineMeshComponent)
    (Collision|SetCollisionEnabled _returnvalue_2 "QueryOnly")
    (Rendering|Material|SetMaterial _returnvalue_2 0 (Variables|Default|GetDynamicMaterial))
    (Rendering|Material|SetVectorParameterValue (Variables|Default|GetDynamicMaterial) "Colour" (Variables|Default|GetSplineColour) :!class /Script/Engine.MaterialInstanceDynamic)
    (Rendering|Material|SetScalarParameterValue (Variables|Default|GetDynamicMaterial) "Strength" (Variables|Default|GetStrength) :!class /Script/Engine.MaterialInstanceDynamic)))