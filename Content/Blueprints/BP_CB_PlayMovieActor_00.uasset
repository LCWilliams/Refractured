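; BP_CB_PlayMovieActor_00 is an actor that plays a full-screen or on-screen movie once its receiver check passes.
; Each Tick it runs CheckReceivers on ReceiverRef; a DoOnce then creates a MoviePlayerWidget for the first player, adds it to the viewport and plays MovieToPlay.
; ResetVideo re-arms the DoOnce so the movie can play again; the IsEndGame branch is empty.
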(event Custom|ResetVideo
  (Utilities|FlowControl|DoOnce false) ; enters at Reset
)

(event EventTick
  (params (DeltaSeconds :type Float%20%28single-precision%29))
  (bind _returnvalue (CallFunction|CheckReceivers (Variables|Config|GetReceiverRef)))
  (if _returnvalue
    (Utilities|FlowControl|DoOnce false
      (:Completed
        (bind _returnvalue_2 (UserInterface|CreateWidget "/Game/Movies/MoviePlayerWidget.MoviePlayerWidget_C" (Game|GetPlayerController 0)))
        (UserInterface|Viewport|AddtoViewport _returnvalue_2 100)
        (Default|PlayMovie _returnvalue_2 (Variables|Config|GetMovieToPlay))
        (if (Variables|Config|GetisEndGame)
          _)))))

(fn ConstructionScript)