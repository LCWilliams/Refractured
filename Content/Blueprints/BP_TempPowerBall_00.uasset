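; Temporary power ball actor that the player picks up, with placeholder level-end logic marked to move into the elevator.
; Tick polls the raycast component's SetObjectActive flag and resets it after a tiny delay.
; The first activation sets HasPowerBall on the player pawn, cached at BeginPlay, and hides the cube.
; Later activations show the cube and print "Level End" if the ball is charged, otherwise print a hint to find the charger.
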(event EventTick
  (params (DeltaSeconds :type Float%20%28single-precision%29))
  (bind _player (Variables|Default|GetPlayer))
  (bind _cube (Variables|Default|GetCube))
  (bind _bp_cb_raycast_component_00 (Variables|Default|GetBP_CB_Raycast_Component_00))
  (if (Variables|/Game/Blueprints/BP_CB_Raycast_Component_00.BP_CB_Raycast_Component_00_C|GetSetObjectActive _bp_cb_raycast_component_00)
    (Utilities|FlowControl|Delay 0.0001)
    ;[1 1 1] Place this in the Elevator
    (Variables|/Game/Blueprints/BP_CB_Raycast_Component_00.BP_CB_Raycast_Component_00_C|SetSetObjectActive _bp_cb_raycast_component_00 false)
    (if (Variables|/Game/Blueprints/BP_CB_PlayerController_00.BP_CB_PlayerController_00_C|GethasPowerBall _player)
      (if (Variables|/Game/Blueprints/BP_CB_PlayerController_00.BP_CB_PlayerController_00_C|GetPowerBallCharged _player)
        (Rendering|SetVisibility _cube true false)
        (Development|PrintString "Level End")
        (else
          (Development|PrintString "Find the Charger")))
      (else
        (Variables|/Game/Blueprints/BP_CB_PlayerController_00.BP_CB_PlayerController_00_C|SethasPowerBall _player true)
        (Rendering|SetVisibility _cube false false)))))

(event EventBeginPlay
  ;[1 1 1] Get Player
  (bind _asbp_cb_player_controller_00 (Utilities|Casting|CastToBP_CB_PlayerController_00 (Game|Player|GetPlayerPawn 0)))
  (Variables|Default|SetPlayer _asbp_cb_player_controller_00))

(fn ConstructionScript)